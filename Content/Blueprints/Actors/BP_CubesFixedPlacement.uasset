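; Actor with three fixed slots (left, right, top) that snap grabbable cubes into place, apparently to build a small stack.
; Each box's begin-overlap event feeds HandleNewCubeOverlap, which ignores non-cube actors and rejects the top slot until two cubes are placed.
; An accepted slot is hidden and loses collision, then the cube handles its own release through OnGetsPlaced, teleports to the slot transform and increments the placed count.
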(event OnComponentBeginOverlap(Box_left)
  (params (OverlappedComponent :type Primitive%20Component%20Object%20Reference) (OtherActor :type Actor%20Object%20Reference) (OtherComp :type Primitive%20Component%20Object%20Reference) (OtherBodyIndex :type Integer) (bFromSweep :type Boolean) (SweepResult :type Hit%20Result%20Structure%20%28by%20ref%29))
  (CallFunction|HandleNewCubeOverlap (Variables|Default|GetBox_left) OtherActor))

(event OnComponentBeginOverlap(Box_right)
  (params (OverlappedComponent :type Primitive%20Component%20Object%20Reference) (OtherActor :type Actor%20Object%20Reference) (OtherComp :type Primitive%20Component%20Object%20Reference) (OtherBodyIndex :type Integer) (bFromSweep :type Boolean) (SweepResult :type Hit%20Result%20Structure%20%28by%20ref%29))
  (CallFunction|HandleNewCubeOverlap (Variables|Default|GetBox_right) OtherActor))

(event OnComponentBeginOverlap(Box_top)
  (params (OverlappedComponent :type Primitive%20Component%20Object%20Reference) (OtherActor :type Actor%20Object%20Reference) (OtherComp :type Primitive%20Component%20Object%20Reference) (OtherBodyIndex :type Integer) (bFromSweep :type Boolean) (SweepResult :type Hit%20Result%20Structure%20%28by%20ref%29))
  (CallFunction|HandleNewCubeOverlap (Variables|Default|GetBox_top) OtherActor))

(fn ConstructionScript)

(fn HandleNewCubeOverlap
  (params (Overlapped%20Component :type Primitive%20Component%20Object%20Reference) (OtherActor :type Actor%20Object%20Reference))
  (bind _asbp_grabbable_cube (Utilities|Casting|CastToBP_Grabbable_Cube OtherActor)
    (:then
      (LocalVariables|SetOverlappedComponent Overlapped%20Component)
      (LocalVariables|SetCube _asbp_grabbable_cube)
      ;[1 1 1] Skip if collision with the top box but 2 bottom boxes are not placed yet
      (if (and (== (LocalVariables|GetOverlappedComponent) (Variables|Default|GetBox_top)) (< (Variables|Default|GetCubesInPlaceCount) 2))
        (return)
        (else
          (Development|SetHiddeninGame (LocalVariables|GetOverlappedComponent) true true)
          (Collision|SetCollisionProfileName (LocalVariables|GetOverlappedComponent) "NoCollision" false :!class /Script/Engine.PrimitiveComponent)
          ;[1 1 1] Letting actor let handle its state: detach if was grabbed and other custom stuff
          (Default|OnGetsPlaced (LocalVariables|GetCube))
          (Transformation|SetWorldLocationAndRotation (Variables|/Script/Engine.Actor|GetRootComponent (LocalVariables|GetCube)) (.location (Transformation|GetWorldTransform (LocalVariables|GetOverlappedComponent))) (.rotation (Transformation|GetWorldTransform (LocalVariables|GetOverlappedComponent))) false true)
          (Variables|Default|SetCubesInPlaceCount (+ (Variables|Default|GetCubesInPlaceCount) 1)))))
    (:CastFailed
      (return))))