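; Grabbable book actor for motion-controller hands, with grab and drop always enabled and no second press needed to drop.
; When a hand can start grabbing it, an idle hand switches animation state, and switches again when that ends unless it is the interacting hand.
; Squared-distance checks pick the grab point closest to the interacting hand and report a hand's nearest distance to the cube or any grab point.
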(event EventOnCanbeGrabbedbyHandStart
  (params (HandMotionController :type VR%20Motion%20Controller%20Hand%20Object%20Reference) (CollidedComponent :type Scene%20Component%20Object%20Reference))
  (if (Class|VRMotionControllerHand|IsHandinIdleState HandMotionController)
    (Class|VRMotionControllerHand|ChangeHandAnimationStateEnum HandMotionController (Utilities|Enum|LiteralenumEHandAnimationState "NewEnumerator5"))))

(event EventOnCanbeGrabbedbyHandEnd
  (params (HandMotionController :type VR%20Motion%20Controller%20Hand%20Object%20Reference) (CollidedComponent :type Scene%20Component%20Object%20Reference))
  (if (not (== (Variables|Default|GetInteractingHand) HandMotionController))
    (Class|VRMotionControllerHand|ChangeHandAnimationStateEnum HandMotionController (Utilities|Enum|LiteralenumEHandAnimationState "NewEnumerator4"))))

(event EventOnGrab
  (params (HandMotionController :type VR%20Motion%20Controller%20Hand%20Object%20Reference)))

(event EventOnDrop
  (params (HandMotionController :type VR%20Motion%20Controller%20Hand%20Object%20Reference)))

(fn ConstructionScript)

(fn GetClosestPointIndextoHand
  (LocalVariables|SetHandLocation (Transformation|GetWorldLocation (Class|HandActor|GetCollisionSphereComponent (Variables|/Script/projectVRBasics.VRMotionControllerHand|GetHandActor (Variables|Default|GetInteractingHand)))))
  (LocalVariables|SetDistance (Class|KismetMathLibrary|VectorDistanceSquared (Transformation|GetWorldLocation (Utilities|Array|Get(acopy) (Variables|Default|GetGrabPointsArray))) (LocalVariables|GetHandLocation)))
  (for (_array_element _array_index) (Variables|Default|GetGrabPointsArray)
    (if (not (== _array_index 0))
      (if (< (Class|KismetMathLibrary|VectorDistanceSquared (LocalVariables|GetHandLocation) (Transformation|GetWorldLocation _array_element)) (LocalVariables|GetDistance))
        (LocalVariables|SetChosenIndex _array_index)
        (LocalVariables|SetDistance (Class|KismetMathLibrary|VectorDistanceSquared (LocalVariables|GetHandLocation) (Transformation|GetWorldLocation _array_element))))))
  (return (LocalVariables|GetChosenIndex)))

(fn GetWorldSquaredDistancetoMotionController
  (params (HandMotionController :type VR%20Motion%20Controller%20Hand%20Object%20Reference))
  (bind _handactor (Variables|/Script/projectVRBasics.VRMotionControllerHand|GetHandActor HandMotionController))
  (bind _returnvalue (Class|HandActor|GetCollisionSphereComponent _handactor))
  (bind _returnvalue_2 (Transformation|GetWorldLocation _returnvalue))
  (LocalVariables|SetFinalDistance (Class|KismetMathLibrary|VectorDistanceSquared (Transformation|GetWorldLocation (Variables|Default|GetCube)) _returnvalue_2))
  (for _array_element (Variables|Default|GetGrabPointsArray)
    (if (< (Class|KismetMathLibrary|VectorDistanceSquared (Transformation|GetWorldLocation _array_element) _returnvalue_2) (LocalVariables|GetFinalDistance))
      (LocalVariables|SetFinalDistance (Class|KismetMathLibrary|VectorDistanceSquared (Transformation|GetWorldLocation _array_element) _returnvalue_2))))
  (return (LocalVariables|GetFinalDistance)))

(fn IsDropDisabled
  (return false))

(fn IsGrabDisabled
  (return false))

(fn IsRequiresSecondButtonPresstoDrop
  (return false))