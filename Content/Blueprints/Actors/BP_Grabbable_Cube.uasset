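; VR grabbable physics cube that a motion controller hand can pick up, pass to the other hand, throw or place.
; On grab it finds the edge component nearest the hand and attaches using an offset requested for that edge and hand side.
; Hand drops restore physics and pass on hand velocity.
; Placement releases it without a throw, then disables physics and grab collision so it stays put.
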(event EventOnGrab
  (params (HandMotionController :type VR%20Motion%20Controller%20Hand%20Object%20Reference))
  (Utilities|IsValid (Variables|Default|GetInteractingHand)
    (:Is%20Valid
      ;[1 1 1] Trying to grab this actor from other hand
      (if (not (Variables|/Script/projectVRBasics.VRMotionControllerHand|GetbIsAttachmentIsInTransitionToHand (Variables|Default|GetInteractingHand)))
        (Class|VRMotionControllerHand|TrytoReleaseGrabbedActor (Variables|Default|GetInteractingHand) false)
        (bind _output_get (Variables|Default|SetInteractingHand HandMotionController :!label _label))
        (Class|VRMotionControllerHand|ChangeHandAnimationStateEnum _output_get (Utilities|Enum|LiteralenumEHandAnimationState "NewEnumerator6"))
        (Physics|SetSimulatePhysics (Variables|Default|GetCube) false)
        ;[1 1 1] Setting relative to hand location depending on closest edge and hand type (left or right, their skeletal meshes are completely different)
        (bind _closestegdescenecomponent (CallFunction|GetClosestEdgetoHand))
        (bind _relativetransform (CallFunction|GetLocationtoAttachto (Class|VirtualRealityMotionController|IsRightHandController (Variables|Default|GetInteractingHand)) _closestegdescenecomponent))
        (Class|VRMotionControllerHand|StartMovingActortoHandforAttachment (Variables|Default|GetInteractingHand) self (.location _relativetransform) (.rotation _relativetransform))))
    (:Is%20Not%20Valid
      (goto _label))))

(event EventOnDrop
  (params (HandMotionController :type VR%20Motion%20Controller%20Hand%20Object%20Reference))
  (bind _cube (Variables|Default|GetCube))
  (Transformation|DetachFromActor "KeepWorld" "KeepWorld" "KeepWorld")
  (if (Variables|Default|GetbDropedByHand)
    ;[1 1 1] Apply velocity if was dropped by hand
    (Physics|SetSimulatePhysics _cube true)
    (Physics|AddImpulse _cube (Transformation|GetVelocity (Variables|/Script/projectVRBasics.VRMotionControllerHand|GetHandActor (Variables|Default|GetInteractingHand))) "None" true)
    (Variables|Default|SetInteractingHand 0)
    (else
      (Variables|Default|SetInteractingHand 0))))

(event EventOnCanbeGrabbedbyHandStart
  (params (HandMotionController :type VR%20Motion%20Controller%20Hand%20Object%20Reference) (CollidedComponent :type Scene%20Component%20Object%20Reference))
  (if (Class|VRMotionControllerHand|IsHandinIdleState HandMotionController)
    (Class|VRMotionControllerHand|ChangeHandAnimationStateEnum HandMotionController (Utilities|Enum|LiteralenumEHandAnimationState "NewEnumerator5"))))

(event EventOnCanbeGrabbedbyHandEnd
  (params (HandMotionController :type VR%20Motion%20Controller%20Hand%20Object%20Reference) (CollidedComponent :type Scene%20Component%20Object%20Reference))
  (Utilities|IsValid (Variables|Default|GetInteractingHand)
    (:Is%20Valid
      (if (not (== (Variables|Default|GetInteractingHand) HandMotionController))
        (Class|VRMotionControllerHand|ChangeHandAnimationStateEnum HandMotionController (Utilities|Enum|LiteralenumEHandAnimationState "NewEnumerator4") :!label _label)))
    (:Is%20Not%20Valid
      (goto _label))))

(event EventBeginPlay
  (bind _edgesarray (Variables|Default|GetEdgesArray))
  ;[1 1 1] Creating array of cube`s egdes
  (Utilities|Array|Add _edgesarray (Variables|Default|GetEdge1))
  (Utilities|Array|Add _edgesarray (Variables|Default|GetEdge2))
  (Utilities|Array|Add _edgesarray (Variables|Default|GetEdge3))
  (Utilities|Array|Add _edgesarray (Variables|Default|GetEdge4))
  (Utilities|Array|Add _edgesarray (Variables|Default|GetEdge5))
  (Utilities|Array|Add _edgesarray (Variables|Default|GetEdge6)))

(fn ConstructionScript)

(fn GetClosestEdgetoHand
  (LocalVariables|SetClosestEgde (Variables|Default|GetEdge1))
  (Utilities|IsValid (Variables|Default|GetInteractingHand)
    (:Is%20Valid
      (bind _output_get (LocalVariables|SetHandLocation (Transformation|GetWorldLocation (Class|HandActor|GetCollisionSphereComponent (Variables|/Script/projectVRBasics.VRMotionControllerHand|GetHandActor (Variables|Default|GetInteractingHand))))))
      (LocalVariables|SetDistanceToHand (Class|KismetMathLibrary|VectorDistanceSquared _output_get (Transformation|GetWorldLocation (LocalVariables|GetClosestEgde))))
      (for (_array_element _array_index) (Variables|Default|GetEdgesArray)
        (if (!= _array_index 0)
          (if (< (Class|KismetMathLibrary|VectorDistanceSquared (Transformation|GetWorldLocation _array_element) (LocalVariables|GetHandLocation)) (LocalVariables|GetDistanceToHand))
            (LocalVariables|SetDistanceToHand (Class|KismetMathLibrary|VectorDistanceSquared (Transformation|GetWorldLocation _array_element) (LocalVariables|GetHandLocation)))
            (LocalVariables|SetClosestEgde _array_element))))
      (return (LocalVariables|GetClosestEgde)))
    (:Is%20Not%20Valid
      (return (LocalVariables|GetClosestEgde)))))

(fn OnGetsPlaced
  (bind _grabcollision (Variables|Default|GetGrabCollision))
  (Utilities|IsValid (Variables|Default|GetInteractingHand)
    (:Is%20Valid
      (Variables|Default|SetbDropedByHand false)
      (Class|VRMotionControllerHand|TrytoReleaseGrabbedActor (Variables|Default|GetInteractingHand) false))
    (:Is%20Not%20Valid
      _))
  (Physics|SetSimulatePhysics (Variables|Default|GetCube) false)
  (Collision|SetCollisionProfileName _grabcollision "NoCollision" true :!class /Script/Engine.PrimitiveComponent)
  (Variables|/Script/Engine.PrimitiveComponent|SetbGenerateOverlapEvents _grabcollision false))

(fn GetLocationtoAttachto
  (params (bRightHand :type Boolean) (Edge :type Scene%20Component%20Object%20Reference))
  (LocalVariables|SetbIsRightHand bRightHand)
  (LocalVariables|SetEdgeComponent Edge)
  (return (Math|Transform|MakeTransform (LocalVariables|GetFinalRelativeLocation) (LocalVariables|GetFinalRelativeRotation) "1,1,1")))

(fn GetWorldSquaredDistancetoMotionController
  (params (HandMotionController :type VR%20Motion%20Controller%20Hand%20Object%20Reference))
  (return (Class|KismetMathLibrary|VectorDistanceSquared (Transformation|GetWorldLocation (Class|HandActor|GetCollisionSphereComponent (Variables|/Script/projectVRBasics.VRMotionControllerHand|GetHandActor HandMotionController))) (Transformation|GetWorldLocation (Variables|Default|GetCube)))))

(fn IsDropDisabled
  (return false))

(fn IsGrabDisabled
  (return false))

(fn IsRequiresSecondButtonPresstoDrop
  (return false))