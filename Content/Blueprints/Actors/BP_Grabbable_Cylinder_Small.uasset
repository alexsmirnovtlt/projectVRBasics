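; BP_Grabbable_Cylinder_Small is a physics cylinder that VR motion controller hands can grab, pass between hands and throw.
; Grabbing turns off physics and has the hand pull it to a per-hand offset, first releasing any holding hand unless that hand's attach transition is running.
; Dropping detaches it, restores physics and applies the hand's velocity as an impulse.
; Grab-range events change hand animation state, and query functions report squared distance and unrestricted grab and drop.
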(event EventOnCanbeGrabbedbyHandStart
  (params (HandMotionController :type VR%20Motion%20Controller%20Hand%20Object%20Reference) (CollidedComponent :type Scene%20Component%20Object%20Reference))
  (if (Class|VRMotionControllerHand|IsHandinIdleState HandMotionController)
    (Class|VRMotionControllerHand|ChangeHandAnimationStateEnum HandMotionController (Utilities|Enum|LiteralenumEHandAnimationState "NewEnumerator5"))))

(event EventOnCanbeGrabbedbyHandEnd
  (params (HandMotionController :type VR%20Motion%20Controller%20Hand%20Object%20Reference) (CollidedComponent :type Scene%20Component%20Object%20Reference))
  (Class|VRMotionControllerHand|ChangeHandAnimationStateEnum HandMotionController (Utilities|Enum|LiteralenumEHandAnimationState "NewEnumerator4")))

(event EventOnGrab
  (params (HandMotionController :type VR%20Motion%20Controller%20Hand%20Object%20Reference))
  (bind _righthandtransform (Variables|Default|GetRightHandTransform))
  (bind _lefthandtransform (Variables|Default|GetLeftHandTransform))
  (Utilities|IsValid (Variables|Default|GetInteractableHand)
    (:Is%20Valid
      ;[1 1 1] Trying to grab this actor from other hand
      (if (not (Variables|/Script/projectVRBasics.VRMotionControllerHand|GetbIsAttachmentIsInTransitionToHand (Variables|Default|GetInteractableHand)))
        (Class|VRMotionControllerHand|TrytoReleaseGrabbedActor (Variables|Default|GetInteractableHand) false)
        (bind _output_get (Variables|Default|SetInteractableHand HandMotionController :!label _label))
        (Class|VRMotionControllerHand|ChangeHandAnimationStateEnum _output_get (Utilities|Enum|LiteralenumEHandAnimationState "NewEnumerator7"))
        (Physics|SetSimulatePhysics (Variables|Default|GetCylinder) false)
        (if (Class|VirtualRealityMotionController|IsRightHandController (Variables|Default|GetInteractableHand))
          (Class|VRMotionControllerHand|StartMovingActortoHandforAttachment (Variables|Default|GetInteractableHand) self (.location _righthandtransform) (.rotation _righthandtransform))
          (else
            (Class|VRMotionControllerHand|StartMovingActortoHandforAttachment (Variables|Default|GetInteractableHand) self (.location _lefthandtransform) (.rotation _lefthandtransform))))))
    (:Is%20Not%20Valid
      (goto _label))))

(event EventOnDrop
  (params (HandMotionController :type VR%20Motion%20Controller%20Hand%20Object%20Reference))
  (bind _handactor (Variables|/Script/projectVRBasics.VRMotionControllerHand|GetHandActor HandMotionController))
  (bind _cylinder (Variables|Default|GetCylinder))
  (bind _returnvalue (Transformation|GetVelocity _handactor))
  (Transformation|DetachFromActor "KeepWorld" "KeepWorld" "KeepWorld")
  (Variables|Default|SetInteractableHand 0)
  (Physics|SetSimulatePhysics _cylinder true)
  (if (not (Math|Vector|VectorIsNearlyZero _returnvalue))
    (Physics|AddImpulse _cylinder _returnvalue "None" true)))

(fn ConstructionScript)

(fn GetConsumeInputParams
  (return (Variables|Default|GetConsumeInputParams)))

(fn GetWorldSquaredDistancetoMotionController
  (params (HandMotionController :type VR%20Motion%20Controller%20Hand%20Object%20Reference))
  (return (Class|KismetMathLibrary|VectorDistanceSquared (Transformation|GetWorldLocation (Class|HandActor|GetCollisionSphereComponent (Variables|/Script/projectVRBasics.VRMotionControllerHand|GetHandActor HandMotionController))) (Transformation|GetWorldLocation (Variables|Default|GetCylinder)))))

(fn IsDropDisabled
  (return false))

(fn IsGrabDisabled
  (return false))

(fn IsRequiresSecondButtonPresstoDrop
  (return false))