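; Sculpt menu actor that lets a motion controller point at and click its widget UI.
; While pointed at, it creates a WidgetInteraction component on demand, moves it to the controller's pointing transform, and destroys it when pointing ends.
; Trigger press and release are forwarded as left mouse button pointer events, so the widget receives mouse-style input.
; It also exposes its input-consumption parameters through a getter.
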(event EventOnGetPointed
  (params (MotionController :type Virtual%20Reality%20Motion%20Controller%20Object%20Reference) (CollidedComponent :type Scene%20Component%20Object%20Reference) (HitLocation :type Vector :default "0, 0, 0"))
  (bind _returnvalue (Class|VirtualRealityMotionController|GetPointingWorldTransform MotionController))
  ;[1 1 1] When gets pointed, create new WidgetInteraction component and update its location so it will update widget`s pointer location as we are using mouse
  (Utilities|IsValid (Variables|Default|GetWidgetInteractionComponent)
    (:Is%20Valid
      (Transformation|SetWorldTransform (Variables|Default|GetWidgetInteractionComponent) _returnvalue false false))
    (:Is%20Not%20Valid
      (bind _returnvalue_2 (AddComponent|AddWidgetInteractionComponent false _returnvalue 0 0.0))
      (bind _output_get (Variables|Default|SetWidgetInteractionComponent _returnvalue_2))
      (Variables|/Script/UMG.WidgetInteractionComponent|SetInteractionDistance _output_get 5e+02))))

(event EventOnEndPointed
  (params (MotionController :type Virtual%20Reality%20Motion%20Controller%20Object%20Reference))
  (bind _widgetinteractioncomponent (Variables|Default|GetWidgetInteractionComponent))
  (Utilities|IsValid _widgetinteractioncomponent
    (:Is%20Valid
      (Components|DestroyComponent _widgetinteractioncomponent))))

(event EventInputButtonTrigger
  (params (ActionType :type EButtonActionType%20Enum :default "Touched"))
  (bind _widgetinteractioncomponent (Variables|Default|GetWidgetInteractionComponent))
  (Utilities|IsValid (Variables|Default|GetWidgetInteractionComponent)
    (:Is%20Valid
      (switch Utilities|FlowControl|Switch|SwitchonEButtonActionType ActionType
        (:Pressed
          (Class|WidgetInteractionComponent|PressPointerKey _widgetinteractioncomponent "LeftMouseButton"))
        (:ReleasedPress
          (Class|WidgetInteractionComponent|ReleasePointerKey _widgetinteractioncomponent "LeftMouseButton"))))))

(fn ConstructionScript)

(fn GetConsumeInputParams
  (return (Variables|Default|GetConsumeInputParams)))