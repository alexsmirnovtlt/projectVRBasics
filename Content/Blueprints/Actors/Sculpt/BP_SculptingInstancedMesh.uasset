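; Sculpting actor that builds shapes from instanced static meshes placed along world locations passed to it.
; AddNewInstancedActor adds a scaled, unrotated instance only when the location is far enough from the last one, using a squared-distance check.
; BeginPlay creates a dynamic sculpt material, which ChangeColor tints through a vector parameter for all instances at once.
; Destroying the actor clears all instances.
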(event EventDestroyed
  (Components|InstancedStaticMesh|ClearInstances (Variables|Default|GetInstancedStaticMesh)))

(event EventBeginPlay
  (bind _returnvalue (Rendering|Material|CreateDynamicMaterialInstance (Variables|Default|GetInstancedStaticMesh) 0 "/Game/Materials/Sculpting/M_Sculpt_Inst.M_Sculpt_Inst" "None" :!class /Script/Engine.PrimitiveComponent))
  (Variables|Default|SetSculptMaterialInstance _returnvalue))

(fn ConstructionScript)

(fn AddNewInstancedActor
  (params (WorldLocation :type Vector))
  (if (>= (Class|KismetMathLibrary|VectorDistanceSquared WorldLocation (Variables|Default|GetLastActorLocation)) (Variables|Default|GetMinDistanceSqrBetweenInstances))
    (bind _output_get (Variables|Default|SetLastActorLocation WorldLocation))
    (Class|InstancedStaticMeshComponent|AddInstanceWorldSpace (Variables|Default|GetInstancedStaticMesh) (Math|Transform|MakeTransform _output_get "0, 0, 0" (Variables|Default|GetSphereScale)))))

(fn ChangeColor
  (params (RGB :type Vector))
  (Utilities|IsValid (Variables|Default|GetSculptMaterialInstance)
    (:Is%20Valid
      (Rendering|Material|SetVectorParameterValue (Variables|Default|GetSculptMaterialInstance) (Variables|Default|GetMaterialInstanceColorParameterName) (Utilities|Struct|MakeLinearColor (.x RGB) (.y RGB) (.z RGB) 1.0) :!class /Script/Engine.MaterialInstanceDynamic))))