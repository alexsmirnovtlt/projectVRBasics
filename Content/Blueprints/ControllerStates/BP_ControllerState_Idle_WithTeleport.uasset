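; Idle state for a VR motion controller that handles grabbing, snap turning and the entry into teleporting.
; Thumbstick input resolves to a dead-zone-filtered direction: up switches to the teleport location finder state, sideways or down rotates the pawn, optionally behind a camera fade.
; A lock allows one turn per stick push until it recenters.
; Grip grabs and releases actors, while the secondary button temporarily toggles between default hands and Oculus Rift S controllers.
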(event Custom|OnFadeTimerEnd
  ;[1 1 1] Rotating our pawn
  (JoystickInputHandling|HandleRotation (Variables|Private|GetCurrentJoystickDirection))
  (bind _cameramanager (Helpers|GetPlayerCameraManager))
  (CameraFades|StartCameraFade :self _cameramanager :FromAlpha 1.0 :Duration (Variables|Customizable|GetCameraFadeDurationSec)))

(event EventOnStateEnter
  ;[1 1 1] Casting Motion Controller to use Grab and Drop functionality
  (bind _asvrmotion_controller_hand (Utilities|Casting|CastToVRMotionControllerHand (Variables|Default|GetOwningMotionController)))
  (Variables|Default|SetHandMovementController _asvrmotion_controller_hand))

(event EventInputAxisThumbstick
  (params (Horizontal :type Float%20%28single-precision%29) (Vertical :type Float%20%28single-precision%29))
  ;[1 1 1] Axis Thumbstick - Getting Raw X and Y input and setting Direction out of it. Then handling look or teleport
  (Variables|Private|SetAxis_X Horizontal)
  (Variables|Private|SetAxis_Y Vertical)
  (bind _joystickdirection (Helpers|GetJoystickInputDirection))
  (bind _output_get (Variables|Private|SetCurrentJoystickDirection _joystickdirection))
  ;[1 1 1] If we looked left or right and then let go our stick, joystick is no longer locked
  (if (Utilities|Enum|Equal(Enum) _output_get "NewEnumerator4")
    (Variables|Private|SetIsJoystickDirectionLocked false)
    (else
      ;[1 1 1] But if it is locked, do nothing. Action has  already been performed
      (if (not (Variables|Private|GetIsJoystickDirectionLocked))
        (switch Utilities|FlowControl|Switch|SwitchonJoystickInputDirection (Variables|Private|GetCurrentJoystickDirection)
          (:NewEnumerator0
            ;[1 1 1] Changing State To Teleport
            (Class|VirtualRealityMotionController|ChangeState (Variables|Default|GetOwningMotionController) "/Game/Blueprints/ControllerStates/BP_ControllerState_TeleportLocationFinder.BP_ControllerState_TeleportLocationFinder_C" true))
          (:NewEnumerator1
            ;[1 1 1] Rotating our pawn
            (if (Variables|Customizable|GetFadeCameraOnRotation) :!label _label
              (Utilities|Time|SetTimerbyEvent (delegate Custom|OnFadeTimerEnd) (Variables|Customizable|GetCameraFadeDurationSec))
              (Variables|Private|SetIsJoystickDirectionLocked true)
              (bind _cameramanager (Helpers|GetPlayerCameraManager))
              (CameraFades|StartCameraFade :self _cameramanager :ToAlpha 1.0 :Duration (Variables|Customizable|GetCameraFadeDurationSec) :bHoldWhenFinished true)
              (else
                (Variables|Private|SetIsJoystickDirectionLocked true)
                (JoystickInputHandling|HandleRotation (Variables|Private|GetCurrentJoystickDirection)))))
          (:NewEnumerator2
            (goto _label))
          (:NewEnumerator3
            (goto _label)))))))

(event EventInputButtonGrip
  (params (ActionType :type EButtonActionType%20Enum :default "Touched"))
  (bind _handmovementcontroller (Variables|Default|GetHandMovementController))
  (bind _handmovementcontroller_2 (Variables|Default|GetHandMovementController))
  (switch Utilities|FlowControl|Switch|SwitchonEButtonActionType ActionType
    (:Pressed
      (Utilities|IsValid _handmovementcontroller_2
        (:Is%20Valid
          (Class|VRMotionControllerHand|TrytoGrabActor _handmovementcontroller_2))))
    (:ReleasedPress
      (Utilities|IsValid _handmovementcontroller
        (:Is%20Valid
          (Class|VRMotionControllerHand|TrytoReleaseGrabbedActor _handmovementcontroller false))))))

(event EventInputButtonSecondary
  (params (ActionType :type EButtonActionType%20Enum :default "Touched"))
  (bind _owningmotioncontroller (Variables|Default|GetOwningMotionController))
  (bind _owningvrpawn (Variables|/Script/projectVRBasics.VirtualRealityMotionController|GetOwningVRPawn _owningmotioncontroller))
  ;[1 1 1] TMP - Change Hands
  (switch Utilities|FlowControl|Switch|SwitchonEButtonActionType ActionType
    (:ReleasedPress
      (if (Utilities|Name|Equal(Name) (Class|VirtualRealityPawn|GetCurrentControllersTypeName _owningvrpawn) "DefaultHands")
        (Class|VirtualRealityPawn|SwitchMotionControllersbyName _owningvrpawn "Oculus Rift S")
        (else
          (Class|VirtualRealityPawn|SwitchMotionControllersbyName _owningvrpawn "DefaultHands"))))))

(fn GetJoystickInputDirection
  (bind _joystickdeadzonesize (Variables|Customizable|GetJoystickDeadZoneSize))
  (bind _axis_x (Variables|Private|GetAxis_X))
  (bind _axis_y (Variables|Private|GetAxis_Y))
  (bind _returnvalue (>= _axis_x _axis_y))
  (if (and (< (Math|Float|Absolute(Float) (Variables|Private|GetAxis_X)) _joystickdeadzonesize) (< (Math|Float|Absolute(Float) (Variables|Private|GetAxis_Y)) _joystickdeadzonesize))
    (return "NewEnumerator4")
    (elif (>= (Math|Float|Absolute(Float) (Variables|Private|GetAxis_X)) (Math|Float|Absolute(Float) (Variables|Private|GetAxis_Y)))
      (if _returnvalue
        (return "NewEnumerator1")
        (else
          (return "NewEnumerator3")))
      (elif _returnvalue
        (return "NewEnumerator2")
        (else
          (return "NewEnumerator0"))))))

(fn HandleRotation
  (params (Direction :type JoystickInputDirection%20Enum :default "NewEnumerator4"))
  (switch Utilities|FlowControl|Switch|SwitchonJoystickInputDirection Direction
    (:NewEnumerator1
      (LocalVariables|SetAddedRotationYaw (Variables|Customizable|GetSideRotationAngle)))
    (:NewEnumerator2
      (LocalVariables|SetAddedRotationYaw 1.8e+02))
    (:NewEnumerator3
      (LocalVariables|SetAddedRotationYaw (* (Variables|Customizable|GetSideRotationAngle) -1.0))))
  (Class|VirtualRealityPawn|AddCameraYawRotation (Variables|/Script/projectVRBasics.VirtualRealityMotionController|GetOwningVRPawn (Variables|Default|GetOwningMotionController)) (LocalVariables|GetAddedRotationYaw)))

(fn GetPlayerCameraManager
  (Utilities|IsValid (Variables|Private|GetCameraManager)
    (:Is%20Valid
      (return (Variables|Private|GetCameraManager)))
    (:Is%20Not%20Valid
      (bind _asplayer_controller (Utilities|Casting|CastToPlayerController (Pawn|GetController (Variables|/Script/projectVRBasics.VirtualRealityMotionController|GetOwningVRPawn (Variables|Default|GetOwningMotionController)))))
      (bind _output_get (Variables|Private|SetCameraManager (Variables|/Script/Engine.PlayerController|GetPlayerCameraManager _asplayer_controller)))
      (return _output_get))))

(fn GetControllerStateasByte
  (return (Variables|Override|GetState)))