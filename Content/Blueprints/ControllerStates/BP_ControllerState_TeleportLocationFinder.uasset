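; VR motion controller state for aiming and performing a thumbstick-driven teleport.
; On enter it creates a BP_VRTeleportLogic object that owns arc visuals and teleport logic, destroyed on exit.
; Each tick it updates the arc from stick axes, or calls teleport and returns to the default state once the stick re-centers.
; Grip, trigger or thumbstick presses, or the other controller entering a specific state, hide the arc and lock aiming.
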(event EventInputAxisThumbstick
  (params (Horizontal :type Float%20%28single-precision%29) (Vertical :type Float%20%28single-precision%29))
  (Variables|Private|SetAxisX Horizontal)
  (Variables|Private|SetAxisY Vertical))

(event EventOnStateEnter
  ;[1 1 1] Initializing teleport logic that includes actors for visual representation and incapsulated teleport logic itself
  (bind _returnvalue (Game|ConstructObjectfromClass "/Game/Blueprints/ControllerStates/LogicObjects/BP_VRTeleportLogic.BP_VRTeleportLogic_C" self))
  (bind _output_get (Variables|Private|SetTeleportLogic _returnvalue))
  (Class|VRTeleportLogic|Initialize _output_get (Variables|Default|GetOwningMotionController)))

(event EventInputButtonGrip
  (params (ActionType :type EButtonActionType%20Enum :default "Touched"))
  ;[1 1 1] Exit Teleport state if Grip, Trigger of Thumbstick were pressed
  (switch Utilities|FlowControl|Switch|SwitchonEButtonActionType ActionType
    (:Pressed
      (Variables|Private|SetIsJoystickInputLocked true)
      (Class|VRTeleportLogic|HideTeleportArc (Variables|Private|GetTeleportLogic) true))))

(event EventOnStateExit
  ;[1 1 1] Need to destroy everything that this class created
  (Class|VRTeleportLogic|HandleDestruction (Variables|Private|GetTeleportLogic)))

(event EventInputButtonTrigger
  (params (ActionType :type EButtonActionType%20Enum :default "Touched"))
  ;[1 1 1] Exit Teleport state if Grip, Trigger of Thumbstick were pressed
  (switch Utilities|FlowControl|Switch|SwitchonEButtonActionType ActionType
    (:Pressed
      (Variables|Private|SetIsJoystickInputLocked true)
      (Class|VRTeleportLogic|HideTeleportArc (Variables|Private|GetTeleportLogic) true))))

(event EventTick
  (params (DeltaTime :type Float%20%28single-precision%29))
  (bind _joystickdeadzonesize (Variables|Customizable|GetJoystickDeadZoneSize))
  (bind _owningmotioncontroller (Variables|Default|GetOwningMotionController))
  (bind _returnvalue (Class|VirtualRealityMotionController|GetControllerWorldOriginTransform _owningmotioncontroller))
  ;[1 1 1] Check If player let go of joystick
  (if (and (< (Math|Float|Absolute(Float) (Variables|Private|GetAxisX)) _joystickdeadzonesize) (< (Math|Float|Absolute(Float) (Variables|Private|GetAxisY)) _joystickdeadzonesize))
    ;[1 1 1] Perform Teleportation If able and return to Idle state
    (Class|VRTeleportLogic|PerformTeleport (Variables|Private|GetTeleportLogic))
    (Class|VirtualRealityMotionController|ChangetoDefaultState (Variables|Default|GetOwningMotionController) true)
    (else
      ;[1 1 1] Do nothing if teleport state now on another controller or action is locked for some other reason
      (if (not (Variables|Private|GetIsJoystickInputLocked))
        ;[1 1 1] Teleport Arc gets updated by logic that stored in special class for that purpose
        (Class|VRTeleportLogic|UpdateTeleportArc (Variables|Private|GetTeleportLogic) (Variables|Private|GetAxisX) (Variables|Private|GetAxisY) (.location _returnvalue) (.rotation _returnvalue))))))

(event EventInputButtonThumbstick
  (params (ActionType :type EButtonActionType%20Enum :default "Touched"))
  ;[1 1 1] Exit Teleport state if Grip, Trigger of Thumbstick were pressed
  (switch Utilities|FlowControl|Switch|SwitchonEButtonActionType ActionType
    (:Pressed
      (Variables|Private|SetIsJoystickInputLocked true)
      (Class|VRTeleportLogic|HideTeleportArc (Variables|Private|GetTeleportLogic) true))))

(event EventPairedControllerStateChanged
  (params (OtherControllerNewState :type Controller%20State%20Object%20Reference) (bEntered :type Boolean))
  ;[1 1 1] If other controller entered same state as this one, disable input for current state
  (if (and bEntered (Utilities|Enum|Equal(Enum) (Utilities|Enum|ByteToEnumEControllerState (CallFunction|GetControllerStateasByte OtherControllerNewState)) "NewEnumerator1"))
    (Variables|Private|SetIsJoystickInputLocked true)
    (Class|VRTeleportLogic|HideTeleportArc (Variables|Private|GetTeleportLogic) true)))

(fn GetControllerStateasByte
  (return (Variables|Override|GetState)))