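; Controller state for the secondary hand during VR sculpting, showing the sculpt menu and handling locomotion.
; On enter it hides the controller and phantom hand and attaches a spawned BP_SculptMenu to the hand at a left or right specific offset; exit reverses this.
; Thumbstick up switches to a sculpting teleport state, while other directions yaw the pawn behind a camera fade, locked until the stick recenters.
; The teleport logic is copied from BP_ControllerState_Idle_WithTeleport.
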(event Custom|CustomEvent_0
  ;[0.9952 1 0.4496] Logic related to teleportation was copied from  BP_ControllerState_Idle_WithTeleport
  ;;[1 1 1] Rotating our pawn
  (CallFunction|HandleRotation (Variables|Private|GetCurrentJoystickDirection))
  (bind _cameramanager (CallFunction|GetPlayerCameraManager))
  (CameraFades|StartCameraFade :self _cameramanager :FromAlpha 1.0 :Duration (Variables|Customizable|GetCameraFadeDurationSec)))

(event EventOnStateEnter
  (bind _asvrmotion_controller_hand (Utilities|Casting|CastToVRMotionControllerHand (Variables|Default|GetOwningMotionController)))
  (bind _output_get (Variables|Default|SetHandMovementController _asvrmotion_controller_hand))
  (Class|VirtualRealityMotionController|SetControllerVisibility _output_get false)
  (Class|VRMotionControllerHand|SetPhantomHandVisibility _output_get false)
  ;[1 1 1] Spawning Sculpting Widget and attaching it to a hand
  (bind _returnvalue (Class|ControllerState|SpawnActor "/Game/Blueprints/Actors/Sculpt/BP_SculptMenu.BP_SculptMenu_C"))
  (bind _asbp_sculpt_menu (Utilities|Casting|CastToBP_SculptMenu _returnvalue))
  (bind _output_get_2 (Variables|Default|SetSculptUIActor _asbp_sculpt_menu))
  (Transformation|AttachActorToActor _output_get_2 (Variables|/Script/projectVRBasics.VRMotionControllerHand|GetHandActor _output_get) "None" "SnapToTarget" "SnapToTarget" "KeepWorld" false)
  (if (Class|VirtualRealityMotionController|IsRightHandController _output_get)
    (Transformation|SetRelativeTransform (Variables|/Script/Engine.Actor|GetRootComponent _output_get_2) (Math|Transform|MakeTransform (Variables|Default|GetRightHandWidgetLocation) (Variables|Default|GetRightHandWidgetRotation) (Transformation|GetWorldScale (Variables|/Script/Engine.Actor|GetRootComponent _output_get_2))) false true)
    (else
      (Transformation|SetRelativeTransform (Variables|/Script/Engine.Actor|GetRootComponent _output_get_2) (Math|Transform|MakeTransform (Variables|Default|GetLeftHandWidgetLocation) (Variables|Default|GetLeftHandWidgetRotation) (Transformation|GetWorldScale (Variables|/Script/Engine.Actor|GetRootComponent _output_get_2))) false true))))

(event EventInputAxisThumbstick
  (params (Horizontal :type Float%20%28single-precision%29) (Vertical :type Float%20%28single-precision%29))
  ;[0.9952 1 0.4496] Logic related to teleportation was copied from  BP_ControllerState_Idle_WithTeleport
  ;;[1 1 1] Axis Thumbstick - Getting Raw X and Y input and setting Direction out of it. Then handling look or teleport
  (Variables|Private|SetAxis_X Horizontal)
  (Variables|Private|SetAxis_Y Vertical)
  (bind _joystickdirection (CallFunction|GetJoystickInputDirection))
  (bind _output_get (Variables|Private|SetCurrentJoystickDirection _joystickdirection))
  ;;[1 1 1] If we looked left or right and then let go our stick, joystick is no longer locked
  (if (Utilities|Enum|Equal(Enum) _output_get "NewEnumerator4")
    (Variables|Private|SetIsJoystickDirectionLocked false)
    (else
      ;;[1 1 1] But if it is locked, do nothing. Action has  already been performed
      (if (not (Variables|Private|GetIsJoystickDirectionLocked))
        (switch Utilities|FlowControl|Switch|SwitchonJoystickInputDirection (Variables|Private|GetCurrentJoystickDirection)
          (:NewEnumerator0
            ;;[1 1 1] Changing State To Teleport
            (Class|VirtualRealityMotionController|ChangeState (Variables|Default|GetOwningMotionController) "/Game/Blueprints/ControllerStates/Sculpting/BP_ControllerState_TeleportLocationFinder_Sculpting.BP_ControllerState_TeleportLocationFinder_Sculpting_C" true))
          (:NewEnumerator1
            ;;[1 1 1] Rotating our pawn
            (Utilities|Time|SetTimerbyEvent (delegate Custom|CustomEvent_0) (Variables|Customizable|GetCameraFadeDurationSec) :!label _label)
            (Variables|Private|SetIsJoystickDirectionLocked true)
            (bind _cameramanager (CallFunction|GetPlayerCameraManager))
            (CameraFades|StartCameraFade :self _cameramanager :ToAlpha 1.0 :Duration (Variables|Customizable|GetCameraFadeDurationSec) :bHoldWhenFinished true))
          (:NewEnumerator2
            (goto _label))
          (:NewEnumerator3
            (goto _label)))))))

(event EventOnStateExit
  (bind _sculptuiactor (Variables|Default|GetSculptUIActor))
  (bind _handmovementcontroller (Variables|Default|GetHandMovementController))
  (Class|VirtualRealityMotionController|SetControllerVisibility _handmovementcontroller true)
  (Class|VRMotionControllerHand|SetPhantomHandVisibility _handmovementcontroller true)
  (Utilities|IsValid _sculptuiactor
    (:Is%20Valid
      (Actor|DestroyActor _sculptuiactor))))

(fn GetJoystickInputDirection
  (bind _joystickdeadzonesize (Variables|Customizable|GetJoystickDeadZoneSize))
  (bind _axis_x (Variables|Private|GetAxis_X))
  (bind _axis_y (Variables|Private|GetAxis_Y))
  (bind _returnvalue (>= _axis_x _axis_y))
  (if (and (< (Math|Float|Absolute(Float) (Variables|Private|GetAxis_X)) _joystickdeadzonesize) (< (Math|Float|Absolute(Float) (Variables|Private|GetAxis_Y)) _joystickdeadzonesize))
    (return "NewEnumerator4")
    (elif (>= (Math|Float|Absolute(Float) (Variables|Private|GetAxis_X)) (Math|Float|Absolute(Float) (Variables|Private|GetAxis_Y)))
      (if _returnvalue
        (return "NewEnumerator1")
        (else
          (return "NewEnumerator3")))
      (elif _returnvalue
        (return "NewEnumerator2")
        (else
          (return "NewEnumerator0"))))))

(fn GetPlayerCameraManager
  (Utilities|IsValid (Variables|Private|GetCameraManager)
    (:Is%20Valid
      (return (Variables|Private|GetCameraManager)))
    (:Is%20Not%20Valid
      (bind _asplayer_controller (Utilities|Casting|CastToPlayerController (Pawn|GetController (Variables|/Script/projectVRBasics.VirtualRealityMotionController|GetOwningVRPawn (Variables|Default|GetOwningMotionController)))))
      (bind _output_get (Variables|Private|SetCameraManager (Variables|/Script/Engine.PlayerController|GetPlayerCameraManager _asplayer_controller)))
      (return _output_get))))

(fn HandleRotation
  (params (NewParam :type JoystickInputDirection%20Enum :default "NewEnumerator4"))
  (switch Utilities|FlowControl|Switch|SwitchonJoystickInputDirection NewParam
    (:NewEnumerator1
      (LocalVariables|SetAddedRotationYaw (Variables|Customizable|GetSideRotationAngle)))
    (:NewEnumerator2
      (LocalVariables|SetAddedRotationYaw 1.8e+02))
    (:NewEnumerator3
      (LocalVariables|SetAddedRotationYaw (* (Variables|Customizable|GetSideRotationAngle) -1.0))))
  (Class|VirtualRealityPawn|AddCameraYawRotation (Variables|/Script/projectVRBasics.VirtualRealityMotionController|GetOwningVRPawn (Variables|Default|GetOwningMotionController)) (LocalVariables|GetAddedRotationYaw)))