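; BP_DefaultHand_Right is the right-hand motion controller Blueprint with an animated, physics-constrained hand mesh.
; It forwards thumbstick, secondary button, grip and trigger input to ControllerState, while grip and trigger thresholds drive temporary pose flags on BP_DefaultHandAnim.
; On BeginPlay it caches that anim instance and constrains the hand_r bone to MainPhysConstraint.
; Getters expose the arrow's world origin and the spline; mesh hits print the other actor's name.
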(event OnComponentHit(HandMesh)
  (params (HitComponent :type Primitive%20Component%20Object%20Reference) (OtherActor :type Actor%20Object%20Reference) (OtherComp :type Primitive%20Component%20Object%20Reference) (NormalImpulse :type Vector :default "0, 0, 0") (Hit :type Hit%20Result%20Structure%20%28by%20ref%29))
  (Development|PrintString (Utilities|GetDisplayName OtherActor)))

(event EventBeginPlay
  ;[1 1 1] Setting Animator
  (bind _asbp_default_hand_anim (Utilities|Casting|CastToBP_DefaultHandAnim (Components|SkeletalMesh|GetAnimInstance (Variables|Default|GetHandMesh))))
  (Variables|Default|SetHandAnimation _asbp_default_hand_anim)
  (Physics|SetUpPhysConstraint (Variables|Default|GetMainPhysConstraint) "None"))

(event Input|ActionEvents|InputActionButton_Right_Secondary_Press
  (params (Key :type Key%20Structure :default "None"))
  ;[1 1 1] Secondary Button
  (:Released
    (Class|ControllerState|InputButtonSecondary (Variables|Default|GetControllerState) "ReleasedPress")))

(event Input|ActionEvents|InputActionButton_Right_Secondary_Press
  (params (Key :type Key%20Structure :default "None"))
  ;[1 1 1] Secondary Button
  (:Pressed
    (Class|ControllerState|InputButtonSecondary (Variables|Default|GetControllerState) "Pressed")))

(event Input|AxisEvents|InputAxisAxis_Right_Grip
  (params (AxisValue :type Float%20%28single-precision%29))
  ;[1 1 1] Grip
  (Class|ControllerState|InputAxisGrip (Variables|Default|GetControllerState) AxisValue)
  ;[1 1 1] TMP Visual
  (Variables|/Game/Blueprints/Controllers/Hands/BP_DefaultHandAnim.BP_DefaultHandAnim_C|SetbGrip (Variables|Default|GetHandAnimation) (> AxisValue 0.9)))

(event Input|AxisEvents|InputAxisAxis_Right_Trigger
  (params (AxisValue :type Float%20%28single-precision%29))
  ;[1 1 1] Trigger
  (Class|ControllerState|InputAxisTrigger (Variables|Default|GetControllerState) AxisValue)
  ;[1 1 1] TMP visual
  (Variables|/Game/Blueprints/Controllers/Hands/BP_DefaultHandAnim.BP_DefaultHandAnim_C|SetbTrigger (Variables|Default|GetHandAnimation) (> AxisValue 0.9)))

(event Input|AxisEvents|InputAxisAxis_Right_Thumbstick_X
  (params (AxisValue :type Float%20%28single-precision%29))
  ;[1 1 1] Right Controller - Stick Axis
  ;[1 1 1] Input Handling
  (Class|ControllerState|InputAxisThumbstick (Variables|Default|GetControllerState) (Input|AxisValues|GetAxis_Right_Thumbstick_X) (Input|AxisValues|GetAxis_Right_Thumbstick_Y)))

(event Input|AxisEvents|InputAxisAxis_Right_Thumbstick_Y
  (params (AxisValue :type Float%20%28single-precision%29))
  ;[1 1 1] Right Controller - Stick Axis
  ;[1 1 1] Input Handling
  (Class|ControllerState|InputAxisThumbstick (Variables|Default|GetControllerState) (Input|AxisValues|GetAxis_Right_Thumbstick_X) (Input|AxisValues|GetAxis_Right_Thumbstick_Y)))

(fn ConstructionScript)

(fn GetControllerWorldOriginLocation
  (return (Transformation|GetWorldLocation (Variables|Default|GetArrow))))

(fn GetControllerWorldOriginRotation
  (return (Transformation|GetWorldRotation (Variables|Default|GetArrow))))

(fn GetSplineComponent
  (return (Variables|Default|GetSpline)))

(fn SetUpPhysConstraint
  (params (FirstComponent :type Primitive%20Component%20Object%20Reference) (Bone%20Name :type Name))
  (Class|PhysicsConstraintComponent|SetConstrainedComponents (Variables|Default|GetPhysicsConstraint) FirstComponent Bone%20Name (Variables|Default|GetHandMesh) "hand_r"))