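; Left-hand VR controller, a child of the right-hand controller that inherits its logic and swaps in left-specific settings and input.
; BeginPlay sets the left physical hand class, root bone and grip offset before calling the parent.
; Left thumbstick, secondary button, grip and trigger inputs feed ControllerState, with grip and trigger also driving the left hand AnimInstance.
; Empty overrides silence inherited right-hand axis events, and animator functions are overridden for the left AnimBP.
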(event EventBeginPlay
  ;[1 1 1] Everything is from parent class (right hand), but some override functions, variables and input events needed to be changed
  (Variables|Default|SetPhysicalHandClass "/Game/Blueprints/Controllers/Hands/PhysicalHandActors/BP_UnrealHand_Left.BP_UnrealHand_Left_C")
  (Variables|Default|SetPhysicalHandRootBoneName "hand_l")
  (Variables|Default|SetHandTransform_WorldOffset_ToGripSocket (Math|Transform|MakeTransform "14.000000,3.000000,9.000000" "45.000000, 0, 0"))
  (|CallParentFunction))

(event Input|ActionEvents|InputActionButton_Left_Secondary_Press
  (params (Key :type Key%20Structure :default "None"))
  ;[1 1 1] Secondary Button
  (:Released
    (Class|ControllerState|InputButtonSecondary (Variables|Default|GetControllerState) "ReleasedPress")))

(event Input|ActionEvents|InputActionButton_Right_Secondary_Press
  (params (Key :type Key%20Structure :default "None"))
  ;[1 1 1] Our right hand parent already binded those inputs so we must clear them here. Do not forget to change paramerets inside them
)

(event Input|ActionEvents|InputActionButton_Right_Primary_Press
  (params (Key :type Key%20Structure :default "None"))
  ;[1 1 1] Our right hand parent already binded those inputs so we must clear them here. Do not forget to change paramerets inside them
)

(event Input|ActionEvents|InputActionButton_Left_Secondary_Press
  (params (Key :type Key%20Structure :default "None"))
  ;[1 1 1] Secondary Button
  (:Pressed
    (Class|ControllerState|InputButtonSecondary (Variables|Default|GetControllerState) "Pressed")))

(event Input|ActionEvents|InputActionButton_Right_Secondary_Press
  (params (Key :type Key%20Structure :default "None"))
  ;[1 1 1] Our right hand parent already binded those inputs so we must clear them here. Do not forget to change paramerets inside them
)

(event Input|ActionEvents|InputActionButton_Left_Primary_Press
  (params (Key :type Key%20Structure :default "None"))
  ;[1 1 1] TMP
)

(event Input|AxisEvents|InputAxisAxis_Right_Grip
  (params (AxisValue :type Float%20%28single-precision%29))
  ;[1 1 1] Our right hand parent already binded those inputs so we must clear them here. Do not forget to change paramerets inside them
)

(event Input|AxisEvents|InputAxisAxis_Right_Trigger
  (params (AxisValue :type Float%20%28single-precision%29))
  ;[1 1 1] Our right hand parent already binded those inputs so we must clear them here. Do not forget to change paramerets inside them
)

(event Input|AxisEvents|InputAxisAxis_Left_Thumbstick_X
  (params (AxisValue :type Float%20%28single-precision%29))
  ;[1 1 1] Stick Axis
  ;[1 1 1] Input Handling
  (Class|ControllerState|InputAxisThumbstick (Variables|Default|GetControllerState) (Input|AxisValues|GetAxis_Left_Thumbstick_X) (Input|AxisValues|GetAxis_Left_Thumbstick_Y)))

(event Input|AxisEvents|InputAxisAxis_Left_Thumbstick_Y
  (params (AxisValue :type Float%20%28single-precision%29))
  ;[1 1 1] Stick Axis
  ;[1 1 1] Input Handling
  (Class|ControllerState|InputAxisThumbstick (Variables|Default|GetControllerState) (Input|AxisValues|GetAxis_Left_Thumbstick_X) (Input|AxisValues|GetAxis_Left_Thumbstick_Y)))

(event Input|AxisEvents|InputAxisAxis_Right_Thumbstick_X
  (params (AxisValue :type Float%20%28single-precision%29))
  ;[1 1 1] Our right hand parent already binded those inputs so we must clear them here. Do not forget to change paramerets inside them
)

(event Input|AxisEvents|InputAxisAxis_Left_Grip
  (params (AxisValue :type Float%20%28single-precision%29))
  (bind _left_handanimator (Variables|Default|GetLeft_HandAnimator))
  ;[1 1 1] Grip
  (bind _output_get (Variables|Default|SetAxis_Grip AxisValue))
  (Class|ControllerState|InputAxisGrip (Variables|Default|GetControllerState) _output_get)
  ;[1 1 1] Visual - Changing Animation
  (Utilities|IsValid _left_handanimator
    (:Is%20Valid
      (Variables|/Game/Blueprints/Controllers/Hands/AnimationBlueprints/BP_DefaultHandAnim_Left.BP_DefaultHandAnim_Left_C|SetbGrip _left_handanimator (> (Variables|Default|GetAxis_Grip) 0.9))
      (Variables|/Game/Blueprints/Controllers/Hands/AnimationBlueprints/BP_DefaultHandAnim_Left.BP_DefaultHandAnim_Left_C|SetPressedGripValue _left_handanimator (Variables|Default|GetAxis_Grip)))))

(event Input|AxisEvents|InputAxisAxis_Right_Thumbstick_Y
  (params (AxisValue :type Float%20%28single-precision%29))
  ;[1 1 1] Our right hand parent already binded those inputs so we must clear them here. Do not forget to change paramerets inside them
)

(event Input|AxisEvents|InputAxisAxis_Left_Trigger
  (params (AxisValue :type Float%20%28single-precision%29))
  (bind _left_handanimator (Variables|Default|GetLeft_HandAnimator))
  ;[1 1 1] Trigger
  (bind _output_get (Variables|Default|SetAxis_Trigger AxisValue))
  (Class|ControllerState|InputAxisTrigger (Variables|Default|GetControllerState) _output_get)
  ;[1 1 1] Visual - Changing Animation
  (Utilities|IsValid _left_handanimator
    (:Is%20Valid
      (Variables|/Game/Blueprints/Controllers/Hands/AnimationBlueprints/BP_DefaultHandAnim_Left.BP_DefaultHandAnim_Left_C|SetbTrigger _left_handanimator (> (Variables|Default|GetAxis_Trigger) 0.9))
      (Variables|/Game/Blueprints/Controllers/Hands/AnimationBlueprints/BP_DefaultHandAnim_Left.BP_DefaultHandAnim_Left_C|SetPressedTriggerValue _left_handanimator (Variables|Default|GetAxis_Trigger)))))

(fn ConstructionScript
  (|CallParentFunction))

(fn SetHandAnimator
  (bind _physicalhand_rootmesh (Variables|Default|GetPhysicalHand_RootMesh))
  (Utilities|IsValid _physicalhand_rootmesh
    (:Is%20Valid
      (bind _asbp_default_hand_anim_left (Utilities|Casting|CastToBP_DefaultHandAnim_Left (Components|SkeletalMesh|GetAnimInstance _physicalhand_rootmesh)))
      (Variables|Default|SetLeft_HandAnimator _asbp_default_hand_anim_left))))

(fn ChangeHandAnimation
  (params (HandAnimationEnum :type EHandAnimationState%20Enum :default "NewEnumerator4"))
  (bind _left_handanimator (Variables|Default|GetLeft_HandAnimator))
  (Utilities|IsValid _left_handanimator
    (:Is%20Valid
      (Variables|/Game/Blueprints/Controllers/Hands/AnimationBlueprints/BP_DefaultHandAnim_Left.BP_DefaultHandAnim_Left_C|SetHandState _left_handanimator HandAnimationEnum))))