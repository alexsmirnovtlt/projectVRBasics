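; Right-hand VR controller that drives a physics-simulated hand and forwards stick, button, grip and trigger input to ControllerState.
; It spawns the hand as a separate actor and binds it by physics constraint to follow the phantom hand.
; After pawn teleports, the hand jumps to the camera, sweeps to its target and restarts physics to avoid sway.
; Grip and trigger also feed the hand animator; a temporary primary-button binding toggles constraint and collision.
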(event EventOnDoneInitbyPawn
  (Physics|InitializePhysicalHand)
  (Setup|SetHandAnimator))

(event EventDestroyed
  (bind _physicalhand_actor (Variables|HandLogic|GetPhysicalHand_Actor))
  ;[1 1 1] Destroing created hand
  (Utilities|IsValid _physicalhand_actor
    (:Is%20Valid
      (Actor|DestroyActor _physicalhand_actor))))

(event EventBeginPlay
  ;[1 1 1] Hand spawns somewhere on a floor and without physics so we need to teleport it to motion controller location and make it follow it
  (Utilities|FlowControl|Delay (Variables|Customizable|GetPhysicalHandStartAppearDelay))
  (Physics|TeleportHandtoMotionControllerLocation false)
  (Physics|MakeHandFollowMovementController true)
  (Development|SetHiddeninGame (Variables|HandLogic|GetPhysicalHand_RootMesh) false false))

(event EventTick
  (params (DeltaSeconds :type Float%20%28single-precision%29)))

(event EventOnPawnTeleport
  (params (bStarted :type Boolean) (bCameraViewOnly :type Boolean))
  (bind _physicalhand_rootmesh (Variables|HandLogic|GetPhysicalHand_RootMesh))
  ;[1 1 1] Teleport Handling - just after pawn teleport occured we teleport our hand to the camera and then sweep to actual location. After that we disable and reenable physics (without that hands will sway) and wait a little while camera is still fading out from 1 to 0 alpha. If waiting is not an option other case will be breaking constraint on teleport start and reattaching it on teleport end
  (Utilities|IsValid (Variables|HandLogic|GetPhysicalHand_RootMesh)
    (:Is%20Valid
      (if (not bStarted)
        (Physics|TeleportHandtoMotionControllerLocation true)
        (Physics|SetSimulatePhysics _physicalhand_rootmesh false)
        (Utilities|FlowControl|Delay 0.1)
        (Physics|SetSimulatePhysics _physicalhand_rootmesh true)))))

(event Input|ActionEvents|InputActionButton_Right_Secondary_Press
  (params (Key :type Key%20Structure :default "None"))
  ;[1 1 1] Secondary Button
  (:Released
    (Class|ControllerState|InputButtonSecondary (Variables|Default|GetControllerState) "ReleasedPress")))

(event Input|ActionEvents|InputActionButton_Right_Primary_Press
  (params (Key :type Key%20Structure :default "None"))
  ;[1 1 1] TMP
  (:Pressed
    (if (Variables|Protected|GetbHaveActivePhysConstraint)
      (Physics|BreakCurrentConstraint)
      (Physics|EnableHandCollision false)
      (else
        (Physics|EnableHandCollision true)
        (Physics|MakeHandFollowMovementController true)))))

(event Input|ActionEvents|InputActionButton_Right_Secondary_Press
  (params (Key :type Key%20Structure :default "None"))
  ;[1 1 1] Secondary Button
  (:Pressed
    (Class|ControllerState|InputButtonSecondary (Variables|Default|GetControllerState) "Pressed")))

(event Input|AxisEvents|InputAxisAxis_Right_Grip
  (params (AxisValue :type Float%20%28single-precision%29))
  (bind _right_physicalhand_animator (Variables|HandLogic|GetRight_PhysicalHand_Animator))
  ;[1 1 1] Grip
  (bind _output_get (Variables|Protected|SetAxis_Grip AxisValue))
  (Class|ControllerState|InputAxisGrip (Variables|Default|GetControllerState) _output_get)
  ;[1 1 1] Visual - Changing Animation
  (Utilities|IsValid _right_physicalhand_animator
    (:Is%20Valid
      (Variables|/Game/Blueprints/Controllers/Hands/AnimationBlueprints/BP_DefaultHandAnim_Right.BP_DefaultHandAnim_Right_C|SetbGrip _right_physicalhand_animator (> (Variables|Protected|GetAxis_Grip) 0.9))
      (Variables|/Game/Blueprints/Controllers/Hands/AnimationBlueprints/BP_DefaultHandAnim_Right.BP_DefaultHandAnim_Right_C|SetPressedGripValue _right_physicalhand_animator (Variables|Protected|GetAxis_Grip)))))

(event Input|AxisEvents|InputAxisAxis_Right_Trigger
  (params (AxisValue :type Float%20%28single-precision%29))
  (bind _right_physicalhand_animator (Variables|HandLogic|GetRight_PhysicalHand_Animator))
  ;[1 1 1] Trigger
  (bind _output_get (Variables|Protected|SetAxis_Trigger AxisValue))
  (Class|ControllerState|InputAxisTrigger (Variables|Default|GetControllerState) _output_get)
  ;[1 1 1] Visual - Changing Animation
  (Utilities|IsValid _right_physicalhand_animator
    (:Is%20Valid
      (Variables|/Game/Blueprints/Controllers/Hands/AnimationBlueprints/BP_DefaultHandAnim_Right.BP_DefaultHandAnim_Right_C|SetbTrigger _right_physicalhand_animator (> (Variables|Protected|GetAxis_Grip) 0.9))
      (Variables|/Game/Blueprints/Controllers/Hands/AnimationBlueprints/BP_DefaultHandAnim_Right.BP_DefaultHandAnim_Right_C|SetPressedTriggerValue _right_physicalhand_animator (Variables|Protected|GetAxis_Trigger)))))

(event Input|AxisEvents|InputAxisAxis_Right_Thumbstick_X
  (params (AxisValue :type Float%20%28single-precision%29))
  ;[1 1 1] Stick Axis
  ;[1 1 1] Input Handling
  (Class|ControllerState|InputAxisThumbstick (Variables|Default|GetControllerState) (Input|AxisValues|GetAxis_Right_Thumbstick_X) (Input|AxisValues|GetAxis_Right_Thumbstick_Y)))

(event Input|AxisEvents|InputAxisAxis_Right_Thumbstick_Y
  (params (AxisValue :type Float%20%28single-precision%29))
  ;[1 1 1] Stick Axis
  ;[1 1 1] Input Handling
  (Class|ControllerState|InputAxisThumbstick (Variables|Default|GetControllerState) (Input|AxisValues|GetAxis_Right_Thumbstick_X) (Input|AxisValues|GetAxis_Right_Thumbstick_Y)))

(fn ConstructionScript)

(fn GetControllerWorldOriginLocation
  (Utilities|IsValid (Variables|HandLogic|GetPhysicalHand_Arrow)
    (:Is%20Valid
      (return (Transformation|GetWorldLocation (Variables|HandLogic|GetPhysicalHand_Arrow))))
    (:Is%20Not%20Valid
      (return (Transformation|GetWorldLocation (Variables|Default|GetMotionController))))))

(fn GetControllerWorldOriginRotation
  (Utilities|IsValid (Variables|HandLogic|GetPhysicalHand_Arrow)
    (:Is%20Valid
      (return (Transformation|GetWorldRotation (Variables|HandLogic|GetPhysicalHand_Arrow))))
    (:Is%20Not%20Valid
      (return (Transformation|GetWorldRotation (Variables|Default|GetPhantomHand))))))

(fn GetSplineComponent
  (return (Variables|Default|GetSpline)))

(fn InitializePhysicalHand
  (Utilities|FlowControl|Sequence
    (:then_0
      ;[1 1 1] Spawning new hand as a new actor so we will be able to attach and detach it at any moment
      (bind _returnvalue (Game|SpawnActorfromClass (Variables|Customizable|GetPhysicalHandClass) (Transformation|GetWorldTransform (Variables|Default|GetPhantomHand)) "AlwaysSpawn" self (Variables|Default|GetOwningVRPawn)))
      (bind _ashand_actor (Utilities|Casting|CastToHandActor _returnvalue)
        (:then
          (Variables|HandLogic|SetPhysicalHand_Actor _ashand_actor))
        (:CastFailed
          (return))))
    (:then_1
      ;[1 1 1] Trying to get skeletal mesh from hand to get a reference to animator and setup contraint to follow phantom hand
      (bind _asskeletal_mesh_component (Utilities|Casting|CastToSkeletalMeshComponent (Variables|/Script/Engine.Actor|GetRootComponent (Variables|HandLogic|GetPhysicalHand_Actor)))
        (:then
          (bind _output_get (Variables|HandLogic|SetPhysicalHand_RootMesh _asskeletal_mesh_component))
          (Physics|SetSimulatePhysics _output_get false)
          (Development|SetHiddeninGame _output_get true false)
          (Class|PrimitiveComponent|SetMassOverrideinKg _output_get "None" (Variables|Customizable|GetHandMass) true))
        (:CastFailed
          (return))))
    (:then_2
      ;[1 1 1] Finally attaching physical hand
      (Transformation|AttachComponentToComponent (Variables|HandLogic|GetPhysicalHand_Actor) (Variables|Transformation|GetRootComponent) "None" "KeepWorld" "KeepWorld" "KeepWorld" false))
    (:then_3
      ;[1 1 1] Getting Hand`s Arrow to use for teleport visualization
      (Variables|HandLogic|SetPhysicalHand_Arrow (Class|HandActor|GetArrowComponent (Variables|HandLogic|GetPhysicalHand_Actor))))))

(fn MakeHandFollowMovementController
  (params (TeleportHandToRootToSetupConstraint :type Boolean))
  (LocalVariables|SetbNeedTeleportToConstraintRoot TeleportHandToRootToSetupConstraint)
  ;[1 1 1] Breaking current constraint if present
  (if (Variables|Protected|GetbHaveActivePhysConstraint)
    (Class|PhysicsConstraintComponent|BreakConstraint (Variables|Default|GetPhysicsConstraint)))
  (Utilities|IsValid (Variables|HandLogic|GetPhysicalHand_RootMesh)
    (:Is%20Valid
      (Utilities|FlowControl|Sequence
        (:then_0
          (if (LocalVariables|GetbNeedTeleportToConstraintRoot)
            ;[1 1 1] To correctly setup attachment, most of the time we must teleport hand to position that it will follow (our phantom hand), setup attachment and then teleport it back
            (LocalVariables|SetHandMeshCurrentTransform (Transformation|GetWorldTransform (Variables|HandLogic|GetPhysicalHand_RootMesh)))
            (Transformation|SetWorldTransform (Variables|HandLogic|GetPhysicalHand_RootMesh) (Transformation|GetWorldTransform (Variables|Default|GetPhantomHand)) false true)))
        (:then_1
          ;[1 1 1] Constraint Setup
          (Physics|SetSimulatePhysics (Variables|HandLogic|GetPhysicalHand_RootMesh) true)
          (Class|PhysicsConstraintComponent|SetConstrainedComponents (Variables|Default|GetPhysicsConstraint) (Variables|Default|GetFirstConstraintComponent) "None" (Variables|HandLogic|GetPhysicalHand_RootMesh) (Variables|Customizable|GetPhysicalHandRootBoneName))
          (Variables|Protected|SetbHaveActivePhysConstraint true))
        (:then_2
          (if (LocalVariables|GetbNeedTeleportToConstraintRoot)
            ;[1 1 1] Teleporting hand back
            (Transformation|SetWorldTransform (Variables|HandLogic|GetPhysicalHand_RootMesh) (LocalVariables|GetHandMeshCurrentTransform) false true)))))))

(fn BreakCurrentConstraint
  (bind _physicalhand_rootmesh (Variables|HandLogic|GetPhysicalHand_RootMesh))
  (Class|PhysicsConstraintComponent|BreakConstraint (Variables|Default|GetPhysicsConstraint))
  (Variables|Protected|SetbHaveActivePhysConstraint false)
  (Utilities|IsValid _physicalhand_rootmesh
    (:Is%20Valid
      (Physics|SetSimulatePhysics _physicalhand_rootmesh false))))

(fn TeleportHandtoMotionControllerLocation
  (params (MakeSweepCheck :type Boolean))
  (LocalVariables|SetSweepToTarget MakeSweepCheck)
  (if (and (Utilities|IsValid (Variables|HandLogic|GetPhysicalHand_Actor)) (Utilities|IsValid (Variables|HandLogic|GetPhysicalHand_RootMesh)))
    (if (LocalVariables|GetSweepToTarget)
      ;[1 1 1] In this case, we teleport our hand to camera location first and then sweep to target
      (Transformation|SetWorldLocation (Variables|HandLogic|GetPhysicalHand_RootMesh) (Class|VirtualRealityPawn|GetCameraWorldLocation (Variables|Default|GetOwningVRPawn)) false true))
    (Transformation|SetWorldTransform (Variables|HandLogic|GetPhysicalHand_RootMesh) (Transformation|GetWorldTransform (Variables|Default|GetPhantomHand)) (LocalVariables|GetSweepToTarget) true)))

(fn SetHandAnimator
  (bind _physicalhand_rootmesh (Variables|HandLogic|GetPhysicalHand_RootMesh))
  (Utilities|IsValid _physicalhand_rootmesh
    (:Is%20Valid
      (bind _asbp_default_hand_anim_right (Utilities|Casting|CastToBP_DefaultHandAnim_Right (Components|SkeletalMesh|GetAnimInstance _physicalhand_rootmesh)))
      (Variables|HandLogic|SetRight_PhysicalHand_Animator _asbp_default_hand_anim_right))))

(fn EnableHandCollision
  (params (bEnable :type Boolean))
  (bind _physicalhand_rootmesh (Variables|HandLogic|GetPhysicalHand_RootMesh))
  (bind _output_get (LocalVariables|SetEnableCollision bEnable))
  (Utilities|IsValid (Variables|HandLogic|GetPhysicalHand_RootMesh)
    (:Is%20Valid
      (if _output_get
        (Collision|SetCollisionProfileName _physicalhand_rootmesh "PhysicsActor" false :!class /Script/Engine.PrimitiveComponent)
        (Collision|SetCollisionEnabled _physicalhand_rootmesh "QueryAndPhysics")
        (Class|PrimitiveComponent|SetMassOverrideinKg _physicalhand_rootmesh (Variables|Customizable|GetPhysicalHandRootBoneName) (Variables|Customizable|GetHandMass) true)
        (else
          (Collision|SetCollisionProfileName _physicalhand_rootmesh "NoCollision" false :!class /Script/Engine.PrimitiveComponent))))))

(fn ChangeHandAnimation
  (params (HandAnimationEnum :type EHandAnimationState%20Enum :default "NewEnumerator4"))
  (bind _right_physicalhand_animator (Variables|HandLogic|GetRight_PhysicalHand_Animator))
  (Utilities|IsValid _right_physicalhand_animator
    (:Is%20Valid
      (Variables|/Game/Blueprints/Controllers/Hands/AnimationBlueprints/BP_DefaultHandAnim_Right.BP_DefaultHandAnim_Right_C|SetHandState _right_physicalhand_animator HandAnimationEnum))))

(fn PlaceHandatWorldLocation
  (params (WorldLocation :type Vector%20%28by%20ref%29) (WorldRotation :type Rotator%20%28by%20ref%29))
  (Utilities|IsValid (Variables|HandLogic|GetPhysicalHand_RootMesh)
    (:Is%20Valid
      (bind _worldhandtransform (HandLogic|GetWorldHandTransformbySocketWorldTransform WorldLocation WorldRotation))
      (Transformation|SetWorldLocationAndRotation (Variables|HandLogic|GetPhysicalHand_RootMesh) (.location _worldhandtransform) (.rotation _worldhandtransform) false true))))

(fn GetWorldHandTransformbySocketWorldTransform
  (params (WorldSocketLocation :type Vector%20%28by%20ref%29) (WorldSocketRotation :type Rotator%20%28by%20ref%29))
  (bind _grabhandsocketname (Variables|Customizable|GetGrabHandSocketName))
  (bind _physicalhand_rootmesh (Variables|HandLogic|GetPhysicalHand_RootMesh))
  (bind _physicalhandrootbonename (Variables|Customizable|GetPhysicalHandRootBoneName))
  (bind _phantomhand (Variables|Default|GetPhantomHand))
  (bind _returnvalue (Transformation|GetSocketRotation _physicalhand_rootmesh _grabhandsocketname))
  (bind _returnvalue_2 (Transformation|GetSocketRotation _physicalhand_rootmesh _physicalhandrootbonename))
  (bind _relativerotation (Variables|/Script/Engine.SceneComponent|GetRelativeRotation _phantomhand))
  (LocalVariables|SetSocketLocation WorldSocketLocation)
  (LocalVariables|SetSocketRotation WorldSocketRotation)
  (Utilities|IsValid (Variables|HandLogic|GetPhysicalHand_Actor)
    (:Is%20Valid
      (Utilities|FlowControl|Sequence
        (:then_0
          (LocalVariables|SetWorldHandBonesDirection (+ (- (LocalVariables|GetSocketLocation) (Class|KismetAnimationLibrary|DirectionBetweenSockets (Variables|HandLogic|GetPhysicalHand_RootMesh) (Variables|Customizable|GetPhysicalHandRootBoneName) (Variables|Customizable|GetGrabHandSocketName))) (Variables|/Script/Engine.SceneComponent|GetRelativeLocation (Variables|Default|GetPhantomHand))))
          (LocalVariables|SetWorldHandBonesRotation (Math|Rotator|MakeRotator (+ (.roll _returnvalue_2) (.roll _returnvalue) (.roll _relativerotation)) (+ (.pitch _returnvalue_2) (.pitch _returnvalue) (.pitch _relativerotation)) (+ (.yaw _returnvalue_2) (.yaw _returnvalue) (.yaw _relativerotation)))))
        (:then_1
          ;[1 1 1] To correctly place a hand we need to add direction and rotation of root bone and palm bone to it
          (return (Math|Transform|MakeTransform (LocalVariables|GetWorldHandBonesDirection) "0, 0, 0" (Transformation|GetWorldScale (Variables|HandLogic|GetPhysicalHand_RootMesh)))))))
    (:Is%20Not%20Valid
      (return ""))))