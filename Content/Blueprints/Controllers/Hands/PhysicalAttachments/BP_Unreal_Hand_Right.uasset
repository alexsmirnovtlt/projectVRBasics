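; BP_Unreal_Hand_Right is the right-hand Blueprint among the controllers' physical hand attachments.
; It exposes its parts through getter functions: an arrow, a skeletal hand mesh, a grab collision sphere, and the component that grabbed actors attach to.
; The construction script is empty, and the file holds no grab or animation logic of its own.
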(fn ConstructionScript)

(fn GetArrowComponent
  (return (Variables|Default|GetArrow)))

(fn GetSkeletalHandMeshComponent
  (return (Variables|Default|GetSkeletalMesh)))

(fn GetCollisionSphereComponent
  (return (Variables|Default|GetGrabSphere)))

(fn GetActorAttachmentComponent
  (return (Variables|Default|GetLocationToAttachGrabbedActorTo)))