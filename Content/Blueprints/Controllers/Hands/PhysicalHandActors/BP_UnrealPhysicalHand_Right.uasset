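; Right-hand physical VR hand actor built on a skeletal mesh and a VRHandPhysicalAnimation component.
; Its construction script overrides the mesh mass with HandMass, binds the mesh to the physical animation component and sets up its welded bone driver.
; The mesh ticks in PrePhysics, and a getter exposes the Arrow component.
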(fn ConstructionScript
  (bind _vrhandphysicalanimation (Variables|Default|GetVRHandPhysicalAnimation))
  (Class|PrimitiveComponent|SetMassOverrideinKg (Variables|Default|GetSkeletalMesh) "None" (Variables|Customizable|GetHandMass) true)
  (Class|PhysicalAnimationComponent|SetSkeletalMeshComponent _vrhandphysicalanimation (Variables|Default|GetSkeletalMesh))
  (Class|VRHandPhysicalAnimationComponent|SetupWeldedBoneDriver _vrhandphysicalanimation)
  (Components|Tick|SetTickGroup (Variables|Default|GetSkeletalMesh) "TG_PrePhysics"))

(fn GetArrowComponent
  (return (Variables|Default|GetArrow)))