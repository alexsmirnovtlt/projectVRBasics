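; Left Oculus controller Blueprint that animates a controller model's buttons, thumbstick, trigger and grip to mirror player input.
; Input events rotate or offset gimbal components: the stick tilts and depresses, the trigger rotates, the grip slides, and X and Y buttons move when pressed.
; Getter functions expose an Arrow component's world location and rotation as the controller origin, along with a Spline component.
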(event EventInputAxisThumbstick
  (params (Horizontal :type Float%20%28single-precision%29) (Vertical :type Float%20%28single-precision%29))
  ;[1 1 1] Left Controller - Stick Axis
  ;[1 1 1] Vusial Stick Movement
  (Transformation|SetRelativeRotation (Variables|Default|GetGimbal_Thumbstick) (Math|Rotator|MakeRotator (* Vertical (* (Variables|EditableVisualParameters|GetThumbstickVusialMaxRotationDegrees) -1.0)) 0.0 (* Horizontal (Variables|EditableVisualParameters|GetThumbstickVusialMaxRotationDegrees))) false false))

(event EventInputButtonPrimary
  (params (ActionType :type EButtonActionType%20Enum :default "Touched"))
  (bind _gimbal_button_x (Variables|Default|GetGimbal_Button_X))
  ;[1 1 1] Right Controller - Primary Button Press And Release
  (switch Utilities|FlowControl|Switch|SwitchonEButtonActionType ActionType
    (:Pressed
      (Transformation|SetRelativeLocation _gimbal_button_x (Math|Vector|MakeVector 0.0 0.0 0.2) false false))
    (:ReleasedPress
      (Transformation|SetRelativeLocation _gimbal_button_x (Math|Vector|MakeVector 0.0 0.0 0.0) false false))))

(event EventInputButtonSecondary
  (params (ActionType :type EButtonActionType%20Enum :default "Touched"))
  (bind _gimbal_button_y (Variables|Default|GetGimbal_Button_Y))
  ;[1 1 1] Right Controller - Secondary Button Press And Release Visual
  (switch Utilities|FlowControl|Switch|SwitchonEButtonActionType ActionType
    (:Pressed
      (Transformation|SetRelativeLocation _gimbal_button_y (Math|Vector|MakeVector 0.0 0.0 (Variables|EditableVisualParameters|GetPressedButtonZOffset)) false false))
    (:ReleasedPress
      (Transformation|SetRelativeLocation _gimbal_button_y (Math|Vector|MakeVector 0.0 0.0 0.0) false false))))

(event EventInputButtonThumbstick
  (params (ActionType :type EButtonActionType%20Enum :default "Touched"))
  (bind _gimbal_thumbstick (Variables|Default|GetGimbal_Thumbstick))
  ;[1 1 1] Right Controller - Stick Button Press And Touch Input Handling
  (switch Utilities|FlowControl|Switch|SwitchonEButtonActionType ActionType
    (:Pressed
      ;[1 1 1] Press Visual
      (Transformation|SetRelativeLocation _gimbal_thumbstick (Math|Vector|MakeVector 0.0 (Variables|EditableVisualParameters|GetThumbstickButtonPressedLocationOffset) 0.0) false false))
    (:ReleasedPress
      (Transformation|SetRelativeLocation _gimbal_thumbstick (Math|Vector|MakeVector 0.0 0.0 0.0) false false))))

(event EventInputAxisGrip
  (params (Value :type Float%20%28single-precision%29))
  ;[1 1 1] Right Controller - Grip Visual
  (Transformation|SetRelativeLocation (Variables|Default|GetGimbal_Grip) (Math|Vector|MakeVector (* Value (Variables|EditableVisualParameters|GetPressedGripButtonZOffset)) 0.0 0.0) false false))

(event EventInputAxisTrigger
  (params (Value :type Float%20%28single-precision%29))
  ;[1 1 1] Right Controller - Trigger Axis Visual
  (Transformation|SetRelativeRotation (Variables|Default|GetGimbal_Trigger) (Math|Rotator|MakeRotator (* Value (Variables|EditableVisualParameters|GetPressedTriggerButtonXOffsetModifier)) 0.0 0.0) false false))

(fn ConstructionScript)

(fn GetControllerWorldOriginLocation
  (return (Transformation|GetWorldLocation (Variables|Default|GetArrow))))

(fn GetControllerWorldOriginRotation
  (return (Transformation|GetWorldRotation (Variables|Default|GetArrow))))

(fn GetSplineComponent
  (return (Variables|Default|GetSpline)))