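; Right-hand Oculus controller Blueprint that animates its buttons, trigger, grip and thumbstick from player input.
; Input events move or rotate Gimbal components, with trigger and grip axes driving only those visuals.
; Thumbstick axes and press, touch and release states for every control are forwarded to ControllerState.
; An Arrow component supplies the controller's world origin location and rotation through getter functions.
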(event Input|ActionEvents|InputActionButton_Right_Thumbstick_Press
  (params (Key :type Key%20Structure :default "None"))
  (bind _gimbal_thumbstick (Variables|Default|GetGimbal_Thumbstick))
  (bind _controllerstate (Variables|Default|GetControllerState))
  ;[1 1 1] Right Controller - Stick Button Press And Touch Input Handling
  (:Pressed
    (Class|ControllerState|InputButtonThumbstick _controllerstate "Pressed")
    ;[1 1 1] Press Visual
    (Transformation|SetRelativeLocation _gimbal_thumbstick (Math|Vector|MakeVector 0.0 (Variables|Default|GetThumbstickButtonPressedLocationOffset) 0.0) false false))
  (:Released
    (Class|ControllerState|InputButtonThumbstick _controllerstate "ReleasedPress")
    (Transformation|SetRelativeLocation _gimbal_thumbstick (Math|Vector|MakeVector 0.0 0.0 0.0) false false)))

(event Input|ActionEvents|InputActionButton_Right_Thumbstick_Touch
  (params (Key :type Key%20Structure :default "None"))
  (bind _controllerstate (Variables|Default|GetControllerState))
  ;[1 1 1] Right Controller - Stick Button Press And Touch Input Handling
  (:Pressed
    (Class|ControllerState|InputButtonThumbstick _controllerstate "Touched"))
  (:Released
    (Class|ControllerState|InputButtonThumbstick _controllerstate "ReleasedTouch")))

(event Input|ActionEvents|InputActionButton_Right_Grip_Press
  (params (Key :type Key%20Structure :default "None"))
  (bind _controllerstate (Variables|Default|GetControllerState))
  ;[1 1 1] Right Grip - Press And Touch Input Handling
  (:Pressed
    (Class|ControllerState|InputButtonGrip _controllerstate "Pressed"))
  (:Released
    (Class|ControllerState|InputButtonGrip _controllerstate "ReleasedPress")))

(event Input|ActionEvents|InputActionButton_Right_Grip_Touch
  (params (Key :type Key%20Structure :default "None"))
  (bind _controllerstate (Variables|Default|GetControllerState))
  ;[1 1 1] Right Grip - Press And Touch Input Handling
  (:Pressed
    (Class|ControllerState|InputButtonGrip _controllerstate "Touched"))
  (:Released
    (Class|ControllerState|InputButtonGrip _controllerstate "ReleasedTouch")))

(event Input|ActionEvents|InputActionButton_Right_Primary_Press
  (params (Key :type Key%20Structure :default "None"))
  (bind _controllerstate (Variables|Default|GetControllerState))
  (bind _gimbal_button_a (Variables|Default|GetGimbal_Button_A))
  ;[1 1 1] Right Controller - Primary Button Press And Release
  (:Pressed
    (Transformation|SetRelativeLocation _gimbal_button_a (Math|Vector|MakeVector 0.0 0.0 0.2) false false)
    ;[1 1 1] Input Handling
    (Class|ControllerState|InputButtonPrimary _controllerstate "Pressed"))
  (:Released
    (Transformation|SetRelativeLocation _gimbal_button_a (Math|Vector|MakeVector 0.0 0.0 0.0) false false)
    (Class|ControllerState|InputButtonPrimary _controllerstate "ReleasedPress")))

(event Input|ActionEvents|InputActionButton_Right_Secondary_Press
  (params (Key :type Key%20Structure :default "None"))
  (bind _gimbal_button_b (Variables|Default|GetGimbal_Button_B))
  (bind _controllerstate (Variables|Default|GetControllerState))
  ;[1 1 1] Right Controller - Secondary Button Press And Release Visual
  (:Pressed
    (Transformation|SetRelativeLocation _gimbal_button_b (Math|Vector|MakeVector 0.0 0.0 (Variables|Default|GetPressedButtonZOffset)) false false)
    ;[1 1 1] Input Handling
    (Class|ControllerState|InputButtonSecondary _controllerstate "Pressed"))
  (:Released
    (Transformation|SetRelativeLocation _gimbal_button_b (Math|Vector|MakeVector 0.0 0.0 0.0) false false)
    (Class|ControllerState|InputButtonSecondary _controllerstate "ReleasedPress")))

(event Input|ActionEvents|InputActionButton_Right_Primary_Touch
  (params (Key :type Key%20Structure :default "None"))
  (bind _controllerstate (Variables|Default|GetControllerState))
  ;[1 1 1] Right Primary & Secondary Button - Touch And EndTouch Input Handling
  (:Pressed
    (Class|ControllerState|InputButtonPrimary _controllerstate "Touched"))
  (:Released
    (Class|ControllerState|InputButtonPrimary _controllerstate "ReleasedTouch")))

(event Input|ActionEvents|InputActionButton_Right_Secondary_Touch
  (params (Key :type Key%20Structure :default "None"))
  (bind _controllerstate (Variables|Default|GetControllerState))
  ;[1 1 1] Right Primary & Secondary Button - Touch And EndTouch Input Handling
  (:Pressed
    (Class|ControllerState|InputButtonSecondary _controllerstate "Touched"))
  (:Released
    (Class|ControllerState|InputButtonSecondary _controllerstate "ReleasedTouch")))

(event Input|ActionEvents|InputActionButton_Right_Trigger_Press
  (params (Key :type Key%20Structure :default "None"))
  (bind _controllerstate (Variables|Default|GetControllerState))
  ;[1 1 1] Right Trigger - Press and Touch Input Handling
  (:Pressed
    (Class|ControllerState|InputButtonTrigger _controllerstate "Pressed"))
  (:Released
    (Class|ControllerState|InputButtonTrigger _controllerstate "ReleasedPress")))

(event Input|ActionEvents|InputActionButton_Right_Trigger_Touch
  (params (Key :type Key%20Structure :default "None"))
  (bind _controllerstate (Variables|Default|GetControllerState))
  ;[1 1 1] Right Trigger - Press and Touch Input Handling
  (:Pressed
    (Class|ControllerState|InputButtonTrigger _controllerstate "Touched"))
  (:Released
    (Class|ControllerState|InputButtonTrigger _controllerstate "ReleasedTouch")))

(event Input|AxisEvents|InputAxisAxis_Right_Grip
  (params (AxisValue :type Float%20%28single-precision%29))
  ;[1 1 1] Right Controller - Grip Visual
  (Transformation|SetRelativeLocation (Variables|Default|GetGimbal_Grip) (Math|Vector|MakeVector (* AxisValue (Variables|Default|GetPressedGripButtonZOffset)) 0.0 0.0) false false))

(event Input|AxisEvents|InputAxisAxis_Right_Trigger
  (params (AxisValue :type Float%20%28single-precision%29))
  ;[1 1 1] Right Controller - Trigger Axis Visual
  (Transformation|SetRelativeRotation (Variables|Default|GetGimbal_Trigger) (Math|Rotator|MakeRotator (* AxisValue (Variables|Default|GetPressedTriggerButtonXOffsetModifier)) 0.0 0.0) false false))

(event Input|AxisEvents|InputAxisAxis_Right_Thumbstick_X
  (params (AxisValue :type Float%20%28single-precision%29))
  ;[1 1 1] Right Controller - Stick Axis
  ;[1 1 1] Vusial Stick Movement
  (Transformation|SetRelativeRotation (Variables|Default|GetGimbal_Thumbstick) (Math|Rotator|MakeRotator (* (Input|AxisValues|GetAxis_Right_Thumbstick_Y) (* (Variables|Default|GetThumbstickVusialMaxRotationDegrees) -1.0)) 0.0 (* (Input|AxisValues|GetAxis_Right_Thumbstick_X) (Variables|Default|GetThumbstickVusialMaxRotationDegrees))) false false)
  ;[1 1 1] Input Handling
  (Class|ControllerState|InputAxisThumbstick (Variables|Default|GetControllerState) (Input|AxisValues|GetAxis_Right_Thumbstick_X) (Input|AxisValues|GetAxis_Right_Thumbstick_Y)))

(event Input|AxisEvents|InputAxisAxis_Right_Thumbstick_Y
  (params (AxisValue :type Float%20%28single-precision%29))
  ;[1 1 1] Right Controller - Stick Axis
  ;[1 1 1] Vusial Stick Movement
  (Transformation|SetRelativeRotation (Variables|Default|GetGimbal_Thumbstick) (Math|Rotator|MakeRotator (* (Input|AxisValues|GetAxis_Right_Thumbstick_Y) (* (Variables|Default|GetThumbstickVusialMaxRotationDegrees) -1.0)) 0.0 (* (Input|AxisValues|GetAxis_Right_Thumbstick_X) (Variables|Default|GetThumbstickVusialMaxRotationDegrees))) false false)
  ;[1 1 1] Input Handling
  (Class|ControllerState|InputAxisThumbstick (Variables|Default|GetControllerState) (Input|AxisValues|GetAxis_Right_Thumbstick_X) (Input|AxisValues|GetAxis_Right_Thumbstick_Y)))

(fn ConstructionScript)

(fn GetControllerWorldOriginRotation
  (return (Transformation|GetWorldRotation (Variables|Default|GetArrow))))

(fn GetControllerWorldOriginLocation
  (return (Transformation|GetWorldLocation (Variables|Default|GetArrow))))