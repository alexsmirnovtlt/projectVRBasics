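; MeshCheckBox is a grip-test actor whose box trigger snaps the player's right VR hand onto a fixed pose.
; On overlap, if no hand is active, it stores the overlapping actor's BP_HandController_Right owner, breaks its constraint, disables hand collision, changes its animation and places it at the Arrow's transform.
; End overlap does nothing, as the release logic is disconnected, so the active hand is never cleared here.
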(event OnComponentBeginOverlap(Box)
  (params (OverlappedComponent :type Primitive%20Component%20Object%20Reference) (OtherActor :type Actor%20Object%20Reference) (OtherComp :type Primitive%20Component%20Object%20Reference) (OtherBodyIndex :type Integer) (bFromSweep :type Boolean) (SweepResult :type Hit%20Result%20Structure%20%28by%20ref%29))
  (bind _arrow (Variables|Default|GetArrow))
  (Utilities|IsValid (Variables|Default|GetActiveHand)
    (:Is%20Not%20Valid
      (bind _asbp_hand_controller_right (Utilities|Casting|CastToBP_HandController_Right (Components|GetOwner OtherActor)))
      (bind _output_get (Variables|Default|SetActiveHand _asbp_hand_controller_right))
      (Default|BreakCurrentConstraint _output_get)
      (Default|EnableHandCollision (Variables|Default|GetActiveHand) false)
      (Default|ChangeHandAnimation (Variables|Default|GetActiveHand) "NewEnumerator6")
      (Default|PlaceHandatWorldLocation (Variables|Default|GetActiveHand) (Transformation|GetWorldLocation _arrow) (Transformation|GetWorldRotation _arrow)))))

(event OnComponentEndOverlap(Box)
  (params (OverlappedComponent :type Primitive%20Component%20Object%20Reference) (OtherActor :type Actor%20Object%20Reference) (OtherComp :type Primitive%20Component%20Object%20Reference) (OtherBodyIndex :type Integer))
  (Utilities|IsValid (Variables|Default|GetActiveHand)))

(fn ConstructionScript)