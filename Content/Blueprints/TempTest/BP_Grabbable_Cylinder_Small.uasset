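; Test VR grabbable small cylinder that a motion-controller hand can pick up and drop.
; Grabbing releases any previous hand, disables physics and moves the actor to a per-hand attachment transform, while proximity and grab events switch hand animation states.
; Dropping detaches the controller's HandActor and re-enables physics, but the velocity-based throw force is never executed.
; Thumbstick press only prints debug text, and the pointing handlers return zero vectors.
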(event EventOnCanbeGrabbedbyHandStart
  (params (HandMotionController :type VR%20Motion%20Controller%20Hand%20Object%20Reference) (CollidedComponent :type Scene%20Component%20Object%20Reference))
  (Class|VRMotionControllerHand|ChangeHandAnimationStateEnum HandMotionController (Utilities|Enum|LiteralenumEHandAnimationState "NewEnumerator5")))

(event EventOnCanbeGrabbedbyHandEnd
  (params (HandMotionController :type VR%20Motion%20Controller%20Hand%20Object%20Reference) (CollidedComponent :type Scene%20Component%20Object%20Reference))
  (Class|VRMotionControllerHand|ChangeHandAnimationStateEnum HandMotionController (Utilities|Enum|LiteralenumEHandAnimationState "NewEnumerator4")))

(event EventOnFinishedAttachingtoHand)

(event EventInputButtonThumbstick
  (params (ActionType :type EButtonActionType%20Enum :default "Touched"))
  (switch Utilities|FlowControl|Switch|SwitchonEButtonActionType ActionType
    (:Pressed
      (Development|PrintString "PRESS"))))

(event EventOnGrab
  (params (HandMotionController :type VR%20Motion%20Controller%20Hand%20Object%20Reference))
  (bind _righthandtransform (Variables|Default|GetRightHandTransform))
  (bind _lefthandtransform (Variables|Default|GetLeftHandTransform))
  (Utilities|IsValid (Variables|Default|GetInteractableHand)
    (:Is%20Valid
      (Class|VRMotionControllerHand|TrytoReleaseGrabbedActor (Variables|Default|GetInteractableHand) false))
    (:Is%20Not%20Valid
      _))
  (bind _output_get (Variables|Default|SetInteractableHand HandMotionController))
  (Class|VRMotionControllerHand|ChangeHandAnimationStateEnum _output_get (Utilities|Enum|LiteralenumEHandAnimationState "NewEnumerator7"))
  (Physics|SetSimulatePhysics (Variables|Default|GetCylinder) false)
  (if (Class|VirtualRealityMotionController|IsRightHandController (Variables|Default|GetInteractableHand))
    (Class|VRMotionControllerHand|StartMovingActortoHandforAttachment (Variables|Default|GetInteractableHand) self (.location _righthandtransform) (.rotation _righthandtransform))
    (else
      (Class|VRMotionControllerHand|StartMovingActortoHandforAttachment (Variables|Default|GetInteractableHand) self (.location _lefthandtransform) (.rotation _lefthandtransform)))))

(event EventOnDrop
  (params (HandMotionController :type VR%20Motion%20Controller%20Hand%20Object%20Reference))
  (Transformation|DetachFromActor (Variables|/Script/projectVRBasics.VRMotionControllerHand|GetHandActor HandMotionController) "KeepWorld" "KeepWorld" "KeepWorld")
  (Variables|Default|SetInteractableHand 0)
  (Physics|SetSimulatePhysics (Variables|Default|GetCylinder) true))

(fn ConstructionScript)

(fn GetShouldConsumeInput
  (return false))

(fn GetWorldSquaredDistancetoMotionController
  (params (HandMotionController :type VR%20Motion%20Controller%20Hand%20Object%20Reference))
  (return (Class|KismetMathLibrary|VectorDistanceSquared (.location (Class|VirtualRealityMotionController|GetControllerWorldOriginTransform HandMotionController)) (Transformation|GetWorldLocation (Variables|Default|GetCylinder)))))

(fn IsRequiresSecondButtonPresstoDrop
  (return false))

(fn OnHandPointingEnd
  (params (HandMotionController :type VR%20Motion%20Controller%20Hand%20Object%20Reference) (CollidedComponent :type Scene%20Component%20Object%20Reference))
  (return "0, 0, 0"))

(fn OnHandPointingStart
  (params (HandMotionController :type VR%20Motion%20Controller%20Hand%20Object%20Reference) (CollidedComponent :type Scene%20Component%20Object%20Reference))
  (return "0, 0, 0"))