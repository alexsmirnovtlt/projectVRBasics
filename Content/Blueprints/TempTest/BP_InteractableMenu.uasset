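; BP_InteractableMenu is a test Blueprint for a pointable menu that shows a cube as a marker where it is being pointed at.
; OnGetPointed stores the hit location and reveals Cube1, Tick moves the cube to that location while pointed at, and OnEndPointed hides it.
; The thumbstick input event is an empty stub, and GetConsumeInputParams only returns its stored parameters.
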(event EventOnGetPointed
  (params (MotionController :type Virtual%20Reality%20Motion%20Controller%20Object%20Reference) (CollidedComponent :type Scene%20Component%20Object%20Reference) (HitLocation :type Vector :default "0, 0, 0"))
  (if (Variables|Default|GetbCurrentlyPointedAt)
    _
    (else
      (Rendering|SetVisibility (Variables|Default|GetCube1) true false)))
  (Variables|Default|SetbCurrentlyPointedAt true)
  (Variables|Default|SetHitLocation HitLocation))

(event EventOnEndPointed
  (params (MotionController :type Virtual%20Reality%20Motion%20Controller%20Object%20Reference))
  (Variables|Default|SetbCurrentlyPointedAt false)
  (Rendering|SetVisibility (Variables|Default|GetCube1) false false))

(event EventTick
  (params (DeltaSeconds :type Float%20%28single-precision%29))
  (if (Variables|Default|GetbCurrentlyPointedAt)
    (Transformation|SetWorldLocation (Variables|Default|GetCube1) (Variables|Default|GetHitLocation) false false)))

(event EventInputAxisThumbstick
  (params (Horizontal :type Float%20%28single-precision%29) (Vertical :type Float%20%28single-precision%29)))

(fn ConstructionScript)

(fn GetConsumeInputParams
  (return (Variables|Default|GetConsumeInputParams)))