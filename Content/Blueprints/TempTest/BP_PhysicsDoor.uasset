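; VR door that motion-controller hands can grab by its panel or front and back knobs to swing on a physics constraint.
; A per-hand collision map drives hand animations and picks the grabbed collider.
; Grabbing attaches the physical hand, snapping to per-hand knob transforms, and enables door physics.
; Release restores hand following but leaves physics on; the hand-delta force code is unwired.
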(event EventOnHandTick
  (params (HandMotionController :type VR%20Motion%20Controller%20Hand%20Object%20Reference))
  ;[1 1 1] Tick that gets called only when hand is grabbed this door
  (Utilities|IsValid (Variables|HandInteraction|GetInteractingHand)))

(event EventOnHandTeleported
  (params (HandMotionController :type VR%20Motion%20Controller%20Hand%20Object%20Reference))
  ;[1 1 1] Return hand to Hand Controller on Teleport
  (Utilities|IsValid (Variables|HandInteraction|GetInteractingHand)
    (:Is%20Valid
      (Class|VRMotionControllerHand|ChangeHandAnimationStateEnum (Variables|HandInteraction|GetInteractingHand) (Utilities|Enum|LiteralenumEHandAnimationState "NewEnumerator4"))
      (Class|VRMotionControllerHand|TrytoReleaseGrabbedActor HandMotionController true))))

(event EventOnCanbeGrabbedbyHandStart
  (params (HandMotionController :type VR%20Motion%20Controller%20Hand%20Object%20Reference) (CollidedComponent :type Scene%20Component%20Object%20Reference))
  ;[1 1 1] Update animation of hands when they are colliding with the door
  (Utilities|IsValid CollidedComponent
    (:Is%20Valid
      (GeneralLogic|HandleHandEnter HandMotionController CollidedComponent))))

(event EventOnCanbeGrabbedbyHandEnd
  (params (HandMotionController :type VR%20Motion%20Controller%20Hand%20Object%20Reference) (CollidedComponent :type Scene%20Component%20Object%20Reference))
  ;[1 1 1] Update animation of hands when they are colliding with the door
  (GeneralLogic|HandleHandExit HandMotionController CollidedComponent))

(event EventOnGrab
  (params (HandMotionController :type VR%20Motion%20Controller%20Hand%20Object%20Reference))
  ;[1 1 1] When collided hand send event that it wants to grab or release
  (Utilities|IsValid (Variables|HandInteraction|GetInteractingHand)
    (:Is%20Not%20Valid
      (GeneralLogic|HandleHandGrab HandMotionController))))

(event EventOnDrop
  (params (HandMotionController :type VR%20Motion%20Controller%20Hand%20Object%20Reference))
  ;[1 1 1] When collided hand send event that it wants to grab or release
  (Utilities|IsValid (Variables|HandInteraction|GetInteractingHand)
    (:Is%20Valid
      (if (== (Variables|HandInteraction|GetInteractingHand) HandMotionController)
        (GeneralLogic|HandleHandDrop)))))

(fn ConstructionScript)

(fn EnableDoorPhysics
  (params (bEnable :type Boolean))
  (if bEnable
    (if (not (Variables|Default|GetbDoorPhysicsEnabled))
      (Collision|SetCollisionProfileName (Variables|Default|GetDoorFrame) "NoCollision" true :!class /Script/Engine.PrimitiveComponent)
      (Physics|SetSimulatePhysics (Variables|Default|GetDoor) true)
      (Class|PhysicsConstraintComponent|SetConstrainedComponents (Variables|Default|GetPhysicsConstraint) (Variables|Default|GetHinge) "None" (Variables|Default|GetDoor) "None")
      (Variables|Default|SetbDoorPhysicsEnabled true))
    (else
      (Collision|SetCollisionProfileName (Variables|Default|GetDoorFrame) "BlockAll" true :!class /Script/Engine.PrimitiveComponent)
      (Class|PhysicsConstraintComponent|BreakConstraint (Variables|Default|GetPhysicsConstraint))
      (Physics|SetSimulatePhysics (Variables|Default|GetDoor) false)
      (Variables|Default|SetbDoorPhysicsEnabled false))))

(fn HandleHandEnter
  (params (Hand%20Motion%20Controller :type VR%20Motion%20Controller%20Hand%20Object%20Reference) (Collided%20Component :type Scene%20Component%20Object%20Reference))
  (LocalVariables|SetHandController Hand%20Motion%20Controller)
  (LocalVariables|SetSceneCollision Collided%20Component)
  (LocalVariables|SetControllerName (Utilities|GetObjectName (LocalVariables|GetHandController)))
  ;[1 1 1] Is this a first collision for this hand
  (if (not (Utilities|Map|Contains (Variables|Default|GetHandControllersInCollision_Map) (LocalVariables|GetControllerName)))
    _
    (else
      ;[1 1 1] Remove if there was already another collision
      (Utilities|Map|Remove (Variables|Default|GetHandControllersInCollision_Map) (LocalVariables|GetControllerName))))
  ;[1 1 1] If we are colliding with the door`s frame
  (if (== (LocalVariables|GetSceneCollision) (Variables|Default|GetDoorFrame))
    ;[1 1 1] Return animation state to default and do nothing more
    (Class|VRMotionControllerHand|ChangeHandAnimationStateEnum (LocalVariables|GetHandController) (Utilities|Enum|LiteralenumEHandAnimationState "NewEnumerator4"))
    (else
      (Utilities|Map|Add (Variables|Default|GetHandControllersInCollision_Map) (LocalVariables|GetControllerName) (LocalVariables|GetSceneCollision))
      ;[1 1 1] Changing hand`s animation depending on what component it collided with
      (if (== (LocalVariables|GetSceneCollision) (Variables|Default|GetDoor))
        (Class|VRMotionControllerHand|ChangeHandAnimationStateEnum (LocalVariables|GetHandController) (Utilities|Enum|LiteralenumEHandAnimationState "NewEnumerator6"))
        (else
          (Class|VRMotionControllerHand|ChangeHandAnimationStateEnum (LocalVariables|GetHandController) (Utilities|Enum|LiteralenumEHandAnimationState "NewEnumerator5")))))))

(fn HandleHandExit
  (params (HandController :type VR%20Motion%20Controller%20Hand%20Object%20Reference) (Collided%20Component :type Scene%20Component%20Object%20Reference))
  (bind _output_get (LocalVariables|SetController HandController))
  (LocalVariables|SetControllerName (Utilities|GetObjectName _output_get))
  (LocalVariables|SetComponent Collided%20Component)
  (if (Utilities|Map|Contains (Variables|Default|GetHandControllersInCollision_Map) (LocalVariables|GetControllerName))
    ;[1 1 1] Changing to default animation only if it is the same collision that hand is entered before. Otherwise hand animation was handled in Handle_Hand_Enter()
    (if (== (LocalVariables|GetComponent) (.Value (Utilities|Map|Find (Variables|Default|GetHandControllersInCollision_Map) (LocalVariables|GetControllerName))))
      (Class|VRMotionControllerHand|ChangeHandAnimationStateEnum (LocalVariables|GetController) (Utilities|Enum|LiteralenumEHandAnimationState "NewEnumerator4"))
      (Utilities|Map|Remove (Variables|Default|GetHandControllersInCollision_Map) (LocalVariables|GetControllerName)))
    (else
      (return))))

(fn AttachHandtoDoor
  (bind _interactinghand (Variables|HandInteraction|GetInteractingHand))
  (bind _interactinghand_2 (Variables|HandInteraction|GetInteractingHand))
  (bind _handactor (Variables|/Script/projectVRBasics.VRMotionControllerHand|GetHandActor _interactinghand))
  (bind _handactor_2 (Variables|/Script/projectVRBasics.VRMotionControllerHand|GetHandActor _interactinghand_2))
  (Class|VRMotionControllerHand|StopFollowingPhysConstraint (Variables|HandInteraction|GetInteractingHand))
  (Class|HandActor|ChangeHandPhysProperties _handactor_2 false false)
  (Transformation|AttachComponentToComponent _handactor_2 (Variables|HandInteraction|GetActiveCollider) "None" "KeepWorld" "KeepWorld" "KeepWorld" false)
  (if (not (== (Variables|HandInteraction|GetActiveCollider) (Variables|Default|GetDoor)))
    (if (== (Variables|HandInteraction|GetActiveCollider) (Variables|Default|GetDoorknob_Front))
      (if (Class|VirtualRealityMotionController|IsRightHandController (Variables|HandInteraction|GetInteractingHand))
        (LocalVariables|SetTargetTransform (Variables|HandTransforms|GetRightHand_Front))
        (else
          (LocalVariables|SetTargetTransform (Variables|HandTransforms|GetLeftHand_Front))))
      (Transformation|SetActorRelativeTransform _handactor (Math|Transform|MakeTransform (.location (LocalVariables|GetTargetTransform)) (.rotation (LocalVariables|GetTargetTransform)) (Transformation|GetActorScale3D _handactor)) false false :!label _label)
      ;[1 1 1] Setting custom grab animation
      (Class|VRMotionControllerHand|ChangeHandAnimationStateEnum (Variables|HandInteraction|GetInteractingHand) (Utilities|Enum|LiteralenumEHandAnimationState "NewEnumerator7"))
      (elif (== (Variables|HandInteraction|GetActiveCollider) (Variables|Default|GetDoorknob_Back))
        (if (Class|VirtualRealityMotionController|IsRightHandController (Variables|HandInteraction|GetInteractingHand))
          (LocalVariables|SetTargetTransform (Variables|HandTransforms|GetRightHand_Back))
          (goto _label)
          (else
            (LocalVariables|SetTargetTransform (Variables|HandTransforms|GetLeftHand_Back))
            (goto _label)))))))

(fn HandleHandGrab
  (params (GrabbedController :type VR%20Motion%20Controller%20Hand%20Object%20Reference))
  (LocalVariables|SetControllerName (Utilities|GetObjectName GrabbedController))
  (if (.ReturnValue (Utilities|Map|Find (Variables|Default|GetHandControllersInCollision_Map) (LocalVariables|GetControllerName)))
    (Variables|HandInteraction|SetActiveCollider (.Value (Utilities|Map|Find (Variables|Default|GetHandControllersInCollision_Map) (LocalVariables|GetControllerName))))
    (Variables|HandInteraction|SetInteractingHand GrabbedController)
    (Utilities|Map|Remove (Variables|Default|GetHandControllersInCollision_Map) (LocalVariables|GetControllerName))
    (DoorInteraction|AttachHandtoDoor)
    (DoorInteraction|EnableDoorPhysics true)))

(fn HandleHandDrop
  (Class|VRMotionControllerHand|ChangeHandAnimationStateEnum (Variables|HandInteraction|GetInteractingHand) (Utilities|Enum|LiteralenumEHandAnimationState "NewEnumerator4"))
  (Transformation|DetachFromActor (Variables|/Script/projectVRBasics.VRMotionControllerHand|GetHandActor (Variables|HandInteraction|GetInteractingHand)) "KeepWorld" "KeepWorld" "KeepWorld")
  (Class|VRMotionControllerHand|StartFollowingPhysConstraint (Variables|HandInteraction|GetInteractingHand) true)
  (Variables|HandInteraction|SetInteractingHand 0)
  (Variables|HandInteraction|SetActiveCollider 0))

(fn GetConsumeInputParams
  (return (Variables|Default|GetConsumeInputParams)))

(fn GetWorldSquaredDistancetoMotionController
  (params (HandMotionController :type VR%20Motion%20Controller%20Hand%20Object%20Reference))
  (return 0.0))

(fn IsDropDisabled
  (return false))

(fn IsGrabDisabled
  (return false))

(fn IsRequiresSecondButtonPresstoDrop
  (return false))