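; Test cube for VR hand interaction that reports when a hand enters or leaves its Box trigger.
; Box overlap events filter for HandActor and print ENTER or EXIT.
; OnGrab is an empty stub, while GetWorldLocationOfGrabCheck returns the Cube's world location.
; Unconnected leftover nodes hold older hand casts, validity checks and an attach-to-hand call that never run.
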(event OnComponentBeginOverlap(Box)
  (params (OverlappedComponent :type Primitive%20Component%20Object%20Reference) (OtherActor :type Actor%20Object%20Reference) (OtherComp :type Primitive%20Component%20Object%20Reference) (OtherBodyIndex :type Integer) (bFromSweep :type Boolean) (SweepResult :type Hit%20Result%20Structure%20%28by%20ref%29))
  (Utilities|Casting|CastToHandActor OtherActor)
  (Development|PrintString "ENTER"))

(event OnComponentEndOverlap(Box)
  (params (OverlappedComponent :type Primitive%20Component%20Object%20Reference) (OtherActor :type Actor%20Object%20Reference) (OtherComp :type Primitive%20Component%20Object%20Reference) (OtherBodyIndex :type Integer))
  (Utilities|Casting|CastToHandActor OtherActor)
  (Development|PrintString "EXIT"))

(event EventOnGrab
  (params (MotionController :type Virtual%20Reality%20Motion%20Controller%20Object%20Reference) (CollidedComponent :type Scene%20Component%20Object%20Reference)))

(fn ConstructionScript)

(fn GetWorldLocationOfGrabCheck
  (return (Transformation|GetWorldLocation (Variables|Default|GetCube))))